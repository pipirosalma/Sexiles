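; BP_Collar is an equippable collar, filed under chain armors, that marks the player character wearing it as collared.
; On equip, it sets IsCollared on the character's first Ac_AditionalAnimations component, if present.
; On unequip, it releases the character's bound object and clears that component's IsCollared and IsCaptured flags.
; Both events then run the parent equip or unequip logic, even when the owner is not a BasePlayerChar.
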(event `self.OnEquip`
  (params (owner :type "Character Object Reference"))
  (bind _asbase_player_char (cast `/Game/Characters/BasePlayerChar` owner)
    (:`then`
      (bind _returnvalue (`Actor.K2_GetComponentsByClass` _asbase_player_char "/Game/Mods/SexilesMod/ac_AditionalAnimations.ac_AditionalAnimations_C"))
      (if (> (`KismetArrayLibrary.Array_Length` _returnvalue) 0)
        (set `/Game/Mods/SexilesMod/ac_AditionalAnimations.IsCollared` true (`KismetArrayLibrary.Array_Get` _returnvalue))))
    (:`CastFailed`
      _))
  (`parent.OnEquip` owner))

(event `self.OnUnEquip`
  (params (owner :type "Character Object Reference"))
  (bind _asbase_player_char (cast `/Game/Characters/BasePlayerChar` owner)
    (:`then`
      (`/Game/Mods/SexilesMod/Character/SXM_BP_PC.SetBoundObject` _asbase_player_char false (0.0 0.0 0.0) null)
      (bind _returnvalue (`Actor.K2_GetComponentsByClass` _asbase_player_char "/Game/Mods/SexilesMod/ac_AditionalAnimations.ac_AditionalAnimations_C"))
      (if (> (`KismetArrayLibrary.Array_Length` _returnvalue) 0)
        (bind _item (`KismetArrayLibrary.Array_Get` _returnvalue))
        (set `/Game/Mods/SexilesMod/ac_AditionalAnimations.IsCollared` false _item)
        (set `/Game/Mods/SexilesMod/ac_AditionalAnimations.IsCaptured` false _item)))
    (:`CastFailed`
      _))
  (`parent.OnUnEquip` owner))