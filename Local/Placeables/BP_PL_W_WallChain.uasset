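; Placeable wall chain that binds a character to its location when activated as an interactable.
; It takes the victim from the user's offhand rope; without a rope, it releases the current victim or, if none, binds the user.
; Binding unequips the user's rope and, if CollarCheck finds a "Collar" modifier on the victim's equipment, snaps the cable to the victim's neck socket.
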(event `InteractableInterface.InteractableActivate`
  (params (Component :type "PrimitiveComponent Object Reference") (Instigator :type "PlayerController Object Reference") (HitIndex :type Integer))
  (bind _victimactor (`self.VictimActor`))
  (bind _asbase_player_char (cast `/Game/Characters/BasePlayerChar` (`Controller.K2_GetPawn` Instigator))
    (:`then`
      (bind _asbp_rope_1h_new (cast `/Game/Mods/SexilesMod/Weapons/BP_rope_1h_new` (`GameItem.VisualActor` (`/Game/Characters/BaseBPCombat.GetOffhandWeapon` _asbase_player_char)))
        (:`then`
          (bind _output_get (set `self.VictimActor` (`/Game/Mods/SexilesMod/Weapons/BP_rope_1h_new.victimactor` _asbp_rope_1h_new)))
          (bind _asbase_player_char_2 (cast `/Game/Characters/BasePlayerChar` _output_get :!label _label)
            (:`then`
              (`/Game/Mods/SexilesMod/Character/SXM_BP_PC.SetBoundObject` _asbase_player_char_2 true (`self.K2_GetActorLocation`) (`self.Cable`))
              (`/Game/Mods/SexilesMod/Character/SXM_BP_PC.RopeUnequip` _asbase_player_char)
              (bind _collared (`self.CollarCheck` _asbase_player_char_2)
                (:`Completed`
                  (if _collared
                    (`SceneComponent.K2_AttachToComponent` (`self.Cable`) (`KismetArrayLibrary.Array_Get` (`self.K2_GetComponentsByClass` _asbase_player_char_2 "/Script/Engine.SkeletalMeshComponent")) "b_neck_2" "SnapToTarget" "SnapToTarget" "SnapToTarget" true)
                    (`parent.InteractableActivate` Component Instigator HitIndex :!label _label_2)))))
            (:`CastFailed`
              (goto _label_2))))
        (:`CastFailed`
          (`/Engine/EditorBlueprintResources/StandardMacros.IsValid` _victimactor
            (:`Is Valid`
              (bind _asbase_player_char_3 (cast `/Game/Characters/BasePlayerChar` _victimactor)
                (:`then`
                  (`/Game/Mods/SexilesMod/Character/SXM_BP_PC.SetBoundObject` _asbase_player_char_3 false (0.0 0.0 0.0) (`self.Cable`))
                  (set `self.VictimActor` null)
                  (goto _label_2))
                (:`CastFailed`
                  (goto _label_2))))
            (:`Is Not Valid`
              (set `self.VictimActor` (`Controller.K2_GetPawn` Instigator))
              (goto _label))))))
    (:`CastFailed`
      (goto _label_2))))

(fn `UserConstructionScript`
  (`parent.UserConstructionScript`))