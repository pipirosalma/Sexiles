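; Placeable wall restraint for Conan Exiles that locks a player character into a posed, cuffed position at the lock.
; On interaction it takes the instigator's leashed victim, clearing the leash, or otherwise the instigator, then multicasts a snap to the pose point.
; MulticastFunctions toggles the LockedUpInteract flag and re-attaches the cables between hand bones and wall locks.
; Interacting again, or a velocity change detected through the character movement update delegate, releases the victim.
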(event `CustomEvent_0`
  (params (DeltaSeconds :type "Float (double-precision)") (OldLocation :type "Vector Structure") (OldVelocity :type "Vector Structure"))
  (bind _cableleft (`self.CableLeft`))
  (bind _cableright (`self.CableRight`))
  (if (not (== OldVelocity (`self.GetVelocity` (`self.VictimController`))))
    ;[1 1 1] Release
    (bind _asbase_player_char (cast `/Game/Characters/BasePlayerChar` (`Controller.K2_GetPawn` (`self.VictimController`)) :!label _label))
    (remove `Character.OnCharacterMovementUpdated` _asbase_player_char (delegate `CustomEvent_0`))
    (`/Game/Mods/SexilesMod/Character/SXM_BP_PC.Deactivate` (`self.VictimBasePlayer`))
    (`self.MulticastFunctions` true)
    (set `self.VictimController` null)
    (set `self.VictimBasePlayer` null)
    (set `self.ActorInPose` false)
    (`SceneComponent.K2_AttachToComponent` _cableright (`self.LockRight`) "LockRight" "SnapToTarget" "SnapToTarget" "SnapToTarget" true :!label _label_2)
    (`CableComponent.SetAttachEndTo` _cableright self "Cable_R_Help" "Cable_R_Help")
    (`SceneComponent.K2_AttachToComponent` _cableleft (`self.LockLeft`) "LockLeft" "SnapToTarget" "SnapToTarget" "SnapToTarget" true)
    (`CableComponent.SetAttachEndTo` _cableleft self "Cable_L_Help" "Cable_L_Help")))

(event `MulticastFunctions`
  (params (Condition :type Boolean))
  (bind _cableright (`self.CableRight`))
  (bind _cableleft (`self.CableLeft`))
  (bind _item (`KismetArrayLibrary.Array_Get` (`self.K2_GetComponentsByClass` (`self.VictimBasePlayer`) "/Script/Engine.SkeletalMeshComponent")))
  (set `/Game/Mods/SexilesMod/Character/SXM_Component.LockedUpInteract` (not Condition) (`/Game/Mods/SexilesMod/Character/SXM_BP_PC.SXM_Component` (`self.VictimBasePlayer`)))
  (if Condition
    ;[1 1 1] Release
    (`/Game/Mods/SexilesMod/Character/SXM_BP_PC.Deactivate` (`self.VictimBasePlayer`))
    (goto _label_2)
    (else
      ;[1 1 1] Set In pose
      (`SceneComponent.K2_AttachToComponent` _cableright _item "b_R_hand" "SnapToTarget" "SnapToTarget" "SnapToTarget" true :!label _label_3)
      (`SceneComponent.K2_AttachToComponent` _cableleft _item "b_L_hand" "SnapToTarget" "SnapToTarget" "SnapToTarget" true)
      (`CableComponent.SetAttachEndTo` _cableright self "LockRight" "LockRight")
      (`CableComponent.SetAttachEndTo` _cableleft self "LockLeft" "LockLeft"))))

(event `InteractableInterface.InteractableActivate`
  (params (Component :type "PrimitiveComponent Object Reference") (Instigator :type "PlayerController Object Reference") (HitIndex :type Integer))
  (bind _victimbaseplayer (`self.VictimBasePlayer`))
  (bind _victimbaseplayer_2 (`self.VictimBasePlayer`))
  (if (`self.ActorInPose`)
    (goto _label)
    (else
      ;[1 1 1] Set In pose
      (bind _playercharacter (`self.SelectVictim` Instigator))
      (if _playercharacter
        (add `Character.OnCharacterMovementUpdated` _victimbaseplayer (delegate `CustomEvent_0`))
        (set `self.ActorInPose` true)
        ;;[1 0.9601 0.217] RCP Function
        (`/Game/Mods/SexilesMod/Character/SXM_BP_PC.MulticastTransform` _victimbaseplayer_2 (`KismetMathLibrary.MakeTransform` (`KismetMathLibrary.MakeVector` (.x (.location (`SceneComponent.K2_GetComponentToWorld` (`self.BP_BSC_Sit`)))) (.y (.location (`SceneComponent.K2_GetComponentToWorld` (`self.BP_BSC_Sit`)))) (.z (.location (`SceneComponent.K2_GetComponentToWorld` (`Character.CapsuleComponent` _victimbaseplayer))))) (.rotation (`SceneComponent.K2_GetComponentToWorld` (`self.BP_BSC_Sit`))) (.scale (`SceneComponent.K2_GetComponentToWorld` (`self.BP_BSC_Sit`)))))
        (`/Game/Mods/SexilesMod/Character/SXM_BP_PC.Activate` _victimbaseplayer_2 12 false)
        (`self.MulticastFunctions` false)
        (goto _label_3)))))

(fn `SelectVictim`
  (params (InputPin :type "PlayerController Object Reference"))
  (returns (PlayerCharacter :type Boolean))
  (bind _asbase_player_char (cast `/Game/Characters/BasePlayerChar` (`Controller.K2_GetPawn` InputPin))
    (:`then`
      (bind _returnvalue (`self.GetComponentByClass` _asbase_player_char "/Game/Mods/SexilesMod/ActorComponents/ac_SXM_Leash.ac_SXM_Leash_C"))
      (`/Engine/EditorBlueprintResources/StandardMacros.IsValid` _returnvalue
        (:`Is Valid`
          (`/Engine/EditorBlueprintResources/StandardMacros.IsValid` (`/Game/Mods/SexilesMod/ActorComponents/ac_SXM_Leash.SXM Rope Actor` _returnvalue)
            (:`Is Valid`
              (bind _asbase_player_char_2 (cast `/Game/Characters/BasePlayerChar` (`/Game/Mods/SexilesMod/ActorComponents/ac_SXM_Leash.VictimActor` _returnvalue))
                (:`then`
                  (set `self.VictimBasePlayer` _asbase_player_char_2)
                  (bind _asconan_player_controller (cast `ConanPlayerController` (`/Game/Characters/FuncomFunctionLibrary.GetControllerFromActor` _asbase_player_char_2))
                    (:`then`
                      (set `self.VictimController` _asconan_player_controller))
                    (:`CastFailed`
                      _))
                  (`/Game/Mods/SexilesMod/ActorComponents/ac_SXM_Leash.CleanUP` _returnvalue)
                  (return true))
                (:`CastFailed`
                  _)))
            (:`Is Not Valid`
              (set `self.VictimController` InputPin)
              (bind _asbase_player_char_3 (cast `/Game/Characters/BasePlayerChar` (`Controller.K2_GetPawn` InputPin))
                (:`then`
                  (set `self.VictimBasePlayer` _asbase_player_char_3)
                  (return true))
                (:`CastFailed`
                  _)))))
        (:`Is Not Valid`
          _))
      (return false))
    (:`CastFailed`
      (return false))))

(fn `UserConstructionScript`
  (`parent.UserConstructionScript`))