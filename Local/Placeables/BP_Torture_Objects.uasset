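; Placeable torture object that offers a radial interaction menu to release a victim when occupied, or to place a leashed victim or yourself.
; CheckForVictims runs off-server, reading the local player's leash component and storing its victim as a player or humanoid thrall.
; That result decides whether "Place Victim" appears.
; Clicks switch on the entry's UserValue, but no branches are wired and the release and placement events are empty stubs.
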(event `InteractableInterface.InteractableMenu`
  (params (RadialMenu :type "RadialMenu Object Reference") (HitIndex :type Integer))
  (if (`self.Occupied`)
    (bind _returnvalue (`RadialMenu.AddItem` RadialMenu "Release Victim" "" "/Game/Mods/SexilesMod/Textures/icons/T_SXM_Handcuff_Open.T_SXM_Handcuff_Open" "None" -1))
    (set `RadialMenuEntry.UserValue` 0 _returnvalue)
    (else
      (`self.CheckForVictims`)
      (`|ExecutionSequence`
        (:`then_0`
          (`/Game/Systems/BP_MacroGlobal.Or+Branch` (`KismetSystemLibrary.IsValid` (`self.PlayerVictim`)) (`KismetSystemLibrary.IsValid` (`self.ThrallVictim`))
            (:`True`
              (bind _returnvalue_2 (`RadialMenu.AddItem` RadialMenu "Place Victim" "" "/Game/Mods/SexilesMod/Textures/icons/T_SXM_LeashOn.T_SXM_LeashOn" "None" -1))
              (set `RadialMenuEntry.UserValue` 1 _returnvalue_2))))
        (:`then_1`
          (bind _returnvalue_3 (`RadialMenu.AddItem` RadialMenu "Place Yourself" "" "/Game/Mods/SexilesMod/Textures/icons/T_SXM_Handcuff.T_SXM_Handcuff" "None" -1))
          (set `RadialMenuEntry.UserValue` 2 _returnvalue_3)))))
  (add `RadialMenuEntry.SignalClicked` _returnvalue_3 (delegate `SignalClicked`))
  (add `RadialMenuEntry.SignalClicked` _returnvalue (delegate `SignalClicked`))
  (add `RadialMenuEntry.SignalClicked` _returnvalue_2 (delegate `SignalClicked`)))

(event `SignalClicked`
  (params (menuEntry :type "RadialMenuEntry Object Reference"))
  (switch `int` (`RadialMenuEntry.UserValue` menuEntry)))

(event `ReleaseVictim`)

(event `PlacePlayer`)

(event `PlaceThrall`)

(fn `CheckForVictims`
  (if (not (`KismetSystemLibrary.IsServer`))
    (bind _asbase_player_char (cast `/Game/Characters/BasePlayerChar` (`Controller.K2_GetPawn` (`GameplayStatics.GetPlayerController` 0))))
    (bind _returnvalue (`self.GetComponentByClass` _asbase_player_char "/Game/Mods/SexilesMod/ActorComponents/ac_SXM_Leash.ac_SXM_Leash_C"))
    (`/Engine/EditorBlueprintResources/StandardMacros.IsValid` _returnvalue
      (:`Is Valid`
        (`/Engine/EditorBlueprintResources/StandardMacros.IsValid` (`/Game/Mods/SexilesMod/ActorComponents/ac_SXM_Leash.SXM Rope Actor` _returnvalue)
          (:`Is Valid`
            (bind _victimactor (`/Game/Mods/SexilesMod/ActorComponents/ac_SXM_Leash.VictimActor` _returnvalue))
            (`/Engine/EditorBlueprintResources/StandardMacros.IsValid` _victimactor
              (:`Is Valid`
                (bind _asbase_player_char_2 (cast `/Game/Characters/BasePlayerChar` _victimactor)
                  (:`then`
                    (set `self.PlayerVictim` _asbase_player_char_2))
                  (:`CastFailed`
                    (bind _aspersistent_humanoid_npc (cast `/Game/Characters/NPCs/Humanoid/PersistentHumanoidNPC` _victimactor))
                    (set `self.ThrallVictim` _aspersistent_humanoid_npc)))))))))))

(fn `UserConstructionScript`
  (`parent.UserConstructionScript`))