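; Base placeable torture object that holds a player victim in an animated pose and lets another player use them.
; A radial menu offers place, self-place, release or use, based on occupancy, valid animation IDs and the SXM component's active state.
; Victims come from the local pawn's leash component, and using one partners both players' SXM components.
; Thrall handling is placeholder only, and the pose-cycling menu entry is disconnected.
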(event Custom|PlaceVictim
  ;[1 1 1] PlaceVictim
  (Variables|Default|SetSXM_Occupied true)
  (Utilities|IsValid (Variables|Default|GetSXM_PlayerVictim)
    (:Is%20Valid
      (Default|SetActortoTortureObject (Variables|Default|GetSXM_PlayerVictim) (Variables|Default|GetSXM_ObjectPosition))
      (Default|Activate (Variables|Default|GetSXM_PlayerVictim) (Variables|Default|GetSXMAnimDataID) false))
    (:Is%20Not%20Valid
      (Utilities|IsValid (Variables|Default|GetSXM_ThrallVictim)
        (:Is%20Valid
          ;;[1 0 0] Placeholder for Thralls
          (Development|PrintString "Not Implemented Yet"))
        (:Is%20Not%20Valid
          (Variables|Default|SetSXM_ThrallVictim 0)
          (Variables|Default|SetSXM_PlayerVictim 0))))))

(event Custom|PlaceSelf
  (bind _asbase_player_char (CallFunction|GetInteractingBasePlayer))
  ;[1 1 1] PlaceVictim
  (Utilities|IsValid _asbase_player_char
    (:Is%20Valid
      (Variables|Default|SetSXM_PlayerVictim _asbase_player_char)
      (CallFunction|PlaceVictim))))

(event Custom|ResetVictimValues
  ;[1 1 1] Reset Values
  (Variables|Default|SetSXM_Occupied false)
  (Variables|Default|SetSXM_ThrallVictim 0)
  (Variables|Default|SetSXM_PlayerVictim 0))

(event Custom|ChangePose
  (bind _sxmposeanimvariants (Variables|Default|GetSXMPoseAnimVariants))
  ;[1 1 1] Change Pose
  (if (== (Utilities|Array|Length _sxmposeanimvariants) (+ (Utilities|Array|FindItem _sxmposeanimvariants (Variables|Default|GetSXMAnimDataID)) 1))
    (Variables|Default|SetSXMAnimDataID (Utilities|Array|Get(acopy) _sxmposeanimvariants))
    (else
      (Variables|Default|SetSXMAnimDataID (Utilities|Array|Get(acopy) _sxmposeanimvariants (+ (Utilities|Array|FindItem _sxmposeanimvariants (Variables|Default|GetSXMAnimDataID)) 1)))))
  (CallFunction|ReleaseVictim)
  (CallFunction|PlaceVictim))

(event Custom|ReleaseVictim
  (bind _sxm_playervictim (Variables|Default|GetSXM_PlayerVictim))
  ;[1 1 1] Release Victim
  (Utilities|IsValid _sxm_playervictim
    (:Is%20Valid
      (Default|Deactivate _sxm_playervictim))
    (:Is%20Not%20Valid
      (Utilities|IsValid (Variables|Default|GetSXM_ThrallVictim)
        (:Is%20Valid
          ;;[1 0 0] Placeholder for Thralls
          (Development|PrintString "Not Implemented Yet"))
        (:Is%20Not%20Valid
          (CallFunction|ResetVictimValues))))))

(event Custom|UseVictom
  (bind _asbase_player_char (CallFunction|GetInteractingBasePlayer))
  ;[1 1 1] Use Victim
  (Utilities|IsValid _asbase_player_char
    (:Is%20Valid
      (if (!= _asbase_player_char (Variables|Default|GetSXM_PlayerVictim))
        (Utilities|IsValid (Variables|Default|GetSXM_PlayerVictim)
          (:Is%20Valid
            (Default|SetPartnerShip _asbase_player_char (Variables|/Game/Mods/SexilesMod/Character/SXM_BP_PC.SXM_BP_PC_C|GetSXM_Component (Variables|Default|GetSXM_PlayerVictim)))
            (Default|Activate _asbase_player_char (Variables|Default|GetSXMAnimDataID) false))
          (:Is%20Not%20Valid
            (Utilities|IsValid (Variables|Default|GetSXM_ThrallVictim)
              (:Is%20Valid
                ;;[1 0 0] Placeholder for Thralls
                (Development|PrintString "Not Implemented Yet"))
              (:Is%20Not%20Valid
                (Variables|Default|SetSXM_Occupied false)))))))))

(event EventBeginPlay
  (bind _sxmanimdataid (Variables|Default|GetSXMAnimDataID))
  (bind _sxmposeanimvariants (Variables|Default|GetSXMPoseAnimVariants))
  ;[1 0.9013 0.5207] BeginToPlay
  (|CallParentFunction)
  (Variables|Default|SetSXM_ObjectPosition (Transformation|GetWorldTransform (Variables|Default|GetSXM_TorturePositionHelper)))
  (if (not (Utilities|Array|ContainsItem _sxmposeanimvariants _sxmanimdataid))
    (Utilities|Array|Add _sxmposeanimvariants _sxmanimdataid)))

(event Custom|SignalClicked
  (params (menuEntry :type Radial%20Menu%20Entry%20Object%20Reference))
  (switch int (Variables|/Script/ConanSandbox.RadialMenuEntry|GetUserValue menuEntry)
    (:0
      (CallFunction|ReleaseVictim)
      (CallFunction|ResetVictimValues))
    (:1
      (CallFunction|UseVictom))
    (:2
      (CallFunction|PlaceVictim))
    (:3
      (CallFunction|PlaceSelf))
    (:4
      (CallFunction|ChangePose))))

(event EventInteractableMenu
  (params (RadialMenu :type Radial%20Menu%20Object%20Reference) (HitIndex :type Integer))
  (Utilities|FlowControl|Sequence
    (:then_0
      (if (Variables|Default|GetSXM_Occupied)
        (Utilities|SXMCompoActiveCheck
          (:Is%20Valid
            (Utilities|FlowControl|Sequence
              (:then_0
                (bind _returnvalue (Class|RadialMenu|AddItem RadialMenu "Release Victim" "" "/Game/Mods/SexilesMod/Textures/icons/T_SXM_Handcuff_Open.T_SXM_Handcuff_Open" "None" -1))
                (Variables|/Script/ConanSandbox.RadialMenuEntry|SetUserValue _returnvalue 0)
                (EventDispatchers|AssignSignalClicked (stale _returnvalue_3) (delegate Custom|SignalClicked) :!label _label))
              (:then_1
                (if (Utilities|Array|ContainsItem (Variables|Default|GetSXMValidAnimIDs) (Variables|Default|GetSXMAnimDataID))
                  (bind _returnvalue_2 (Class|RadialMenu|AddItem RadialMenu "Use Victim" "" "/Game/Mods/SexilesMod/Textures/icons/T_SXM_ForceAnimation.T_SXM_ForceAnimation" "None" -1))
                  (Variables|/Script/ConanSandbox.RadialMenuEntry|SetUserValue _returnvalue_2 1)
                  (goto _label)))
              (:then_2))))
        (else
          (CallFunction|CheckforVictims)
          (Utilities|FlowControl|Sequence
            (:then_0
              (Utilities|Or+Branch (Utilities|IsValid (Variables|Default|GetSXM_PlayerVictim)) (Utilities|IsValid (Variables|Default|GetSXM_ThrallVictim))
                (:True
                  (bind _returnvalue_3 (Class|RadialMenu|AddItem RadialMenu "Place Victim" "" "/Game/Mods/SexilesMod/Textures/icons/T_SXM_LeashOn.T_SXM_LeashOn" "None" -1))
                  (Variables|/Script/ConanSandbox.RadialMenuEntry|SetUserValue _returnvalue_3 2)
                  (goto _label))))
            (:then_1
              (bind _returnvalue_4 (Class|RadialMenu|AddItem RadialMenu "Place Yourself" "" "/Game/Mods/SexilesMod/Textures/icons/T_SXM_Handcuff.T_SXM_Handcuff" "None" -1))
              (Variables|/Script/ConanSandbox.RadialMenuEntry|SetUserValue _returnvalue_4 3)
              (goto _label))))))
    (:then_1
      (|CallParentFunction RadialMenu HitIndex))))

(fn ConstructionScript
  (|CallParentFunction))

(fn CheckforVictims
  (bind _asbase_player_char (Utilities|Casting|CastToBasePlayerChar (Pawn|GetControlledPawn (Game|GetPlayerController 0))))
  (Utilities|IsValid (Actor|GetComponentbyClass _asbase_player_char "/Game/Mods/SexilesMod/ActorComponents/ac_SXM_Leash.ac_SXM_Leash_C")
    (:Is%20Valid
      (Utilities|IsValid (Variables|/Game/Mods/SexilesMod/ActorComponents/ac_SXM_Leash.ac_SXM_Leash_C|GetSXM%20Rope%20Actor (Actor|GetComponentbyClass _asbase_player_char "/Game/Mods/SexilesMod/ActorComponents/ac_SXM_Leash.ac_SXM_Leash_C"))
        (:Is%20Valid
          (Utilities|IsValid (Variables|/Game/Mods/SexilesMod/ActorComponents/ac_SXM_Leash.ac_SXM_Leash_C|GetVictimActor (Actor|GetComponentbyClass _asbase_player_char "/Game/Mods/SexilesMod/ActorComponents/ac_SXM_Leash.ac_SXM_Leash_C"))
            (:Is%20Valid
              (bind _asbase_player_char_2 (Utilities|Casting|CastToBasePlayerChar (Variables|/Game/Mods/SexilesMod/ActorComponents/ac_SXM_Leash.ac_SXM_Leash_C|GetVictimActor (Actor|GetComponentbyClass _asbase_player_char "/Game/Mods/SexilesMod/ActorComponents/ac_SXM_Leash.ac_SXM_Leash_C")))
                (:then
                  (Variables|Default|SetSXM_PlayerVictim _asbase_player_char_2))
                (:CastFailed
                  (bind _aspersistent_humanoid_npc (Utilities|Casting|CastToPersistentHumanoidNPC (Variables|/Game/Mods/SexilesMod/ActorComponents/ac_SXM_Leash.ac_SXM_Leash_C|GetVictimActor (Actor|GetComponentbyClass _asbase_player_char "/Game/Mods/SexilesMod/ActorComponents/ac_SXM_Leash.ac_SXM_Leash_C"))))
                  (Variables|Default|SetSXM_ThrallVictim _aspersistent_humanoid_npc))))))))))

(fn GetInteractingBasePlayer
  (bind _asbase_player_char (Utilities|Casting|CastToBasePlayerChar (Pawn|GetControlledPawn (Game|GetPlayerController 0))))
  (return _asbase_player_char))