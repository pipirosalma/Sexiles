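; SXM_TO_Pole_BP is a pole variant of a placeable torture object that can hold a victim.
; It extends the parent's PlaceVictim and ReleaseVictim events, calling the parent logic and then showing or hiding RopeMesh so the rope appears only after a victim is placed.
; Construction defers to the parent, and the BeginPlay, overlap and Tick events are disabled stubs.
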(event `self.PlaceVictim`
  (`parent.PlaceVictim`)
  (`SceneComponent.SetVisibility` (`self.RopeMesh`) true false))

(event `self.ReleaseVictim`
  (`parent.ReleaseVictim`)
  (`SceneComponent.SetVisibility` (`self.RopeMesh`) false false))

(fn `UserConstructionScript`
  (`parent.UserConstructionScript`))