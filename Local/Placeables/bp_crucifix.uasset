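; Placeable crucifix that poses a player or NPC thrall on interaction and releases them on the next use.
; SelectVictim takes the player or thrall on the user's SXM leash and cleans it up, otherwise using the interacting player.
; Players play a movement-blocking animation, optionally flying, and are also released by a velocity-change check.
; Thralls are set Dead while posed, then Passive and returned to their saved transform.
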(event `CustomEvent_0`
  (params (DeltaSeconds :type "Float (double-precision)") (OldLocation :type "Vector Structure") (OldVelocity :type "Vector Structure"))
  (if (not (== OldVelocity (`self.GetVelocity` (`self.VictimController`))))
    ;[1 1 1] Release
    (bind _asbase_player_char (cast `/Game/Characters/BasePlayerChar` (`Controller.K2_GetPawn` (`self.VictimController`)) :!label _label))
    (remove `Character.OnCharacterMovementUpdated` _asbase_player_char (delegate `CustomEvent_0`))
    (`CharacterMovementComponent.SetMovementMode` (`Character.CharacterMovement` _asbase_player_char) "MOVE_Walking" 0)
    (`/Game/Mods/SexilesMod/Character/SXM_BP_PC.RCPPlayAnim` :`self` _asbase_player_char :`Stop` true :`NewAnimToPlay` "/Game/Characters/humans/animations/cinematic/Marketing_Crucifix_Pose_F.Marketing_Crucifix_Pose_F")
    (set `self.ActorInPose` false)
    (set `self.VictimController` null)
    (set `self.VictimBasePlayer` null)))

(event `InteractableInterface.InteractableActivate`
  (params (Component :type "PrimitiveComponent Object Reference") (Instigator :type "PlayerController Object Reference") (HitIndex :type Integer))
  (bind _victimbaseplayer (`self.VictimBasePlayer`))
  (bind _thrallreference (`self.ThrallReference`))
  (if (`self.ActorInPose`)
    (if (`self.IsThrall`)
      (set `self.ActorInPose` false)
      (`/Game/Mods/SexilesMod/Character/SXM_BP_PC.RCPPlayAnim_NPC` (`self.VictimBasePlayer`) true null true (`self.ThrallReference`) (`self.ThrallReturnLocation`))
      (`ConanCharacter.SetCharacterState` (`self.ThrallReference`) "Passive")
      (set `self.ThrallReference` null)
      (else
        (goto _label)))
    (else
      ;[1 1 1] Set In pose
      (bind _playercharacter (`self.SelectVictim` Instigator))
      (if _playercharacter
        (add `Character.OnCharacterMovementUpdated` _victimbaseplayer (delegate `CustomEvent_0`))
        (if (`self.NeedToFly`)
          (`CharacterMovementComponent.SetMovementMode` (`Character.CharacterMovement` _victimbaseplayer) "MOVE_Flying" 0)
          (`KismetSystemLibrary.Delay` 0.2))
        (set `self.ActorInPose` true)
        ;;[1 0.9601 0.217] RCP Function
        (`/Game/Mods/SexilesMod/Character/SXM_BP_PC.RCPPlayAnim` (`self.VictimBasePlayer`) false null true (`SceneComponent.K2_GetComponentToWorld` (`self.PoistionHelper`)) (`self.AnimationToPlay`))
        (else
          (set `self.ActorInPose` true)
          (`ConanCharacter.SetCharacterState` (`self.ThrallReference`) "Dead")
          (set `self.ThrallReturnLocation` (`self.GetTransform` _thrallreference))
          (`/Game/Mods/SexilesMod/Character/SXM_BP_PC.RCPPlayAnim_NPC` (`self.VictimBasePlayer`) false "/Game/Characters/humans/animations/cinematic/Marketing_Crucifix_Pose_F.Marketing_Crucifix_Pose_F" true _thrallreference (`SceneComponent.K2_GetComponentToWorld` (`self.PoistionHelper`))))))))

(fn `SelectVictim`
  (params (VictimController :type "PlayerController Object Reference"))
  (returns (PlayerCharacter :type Boolean))
  (bind _returnvalue (`Controller.K2_GetPawn` VictimController))
  (bind _asbase_player_char (cast `/Game/Characters/BasePlayerChar` (`Controller.K2_GetPawn` VictimController))
    (:`then`
      (bind _returnvalue_2 (`self.GetComponentByClass` _asbase_player_char "/Game/Mods/SexilesMod/ActorComponents/ac_SXM_Leash.ac_SXM_Leash_C"))
      (`/Engine/EditorBlueprintResources/StandardMacros.IsValid` _returnvalue_2
        (:`Is Valid`
          (`/Engine/EditorBlueprintResources/StandardMacros.IsValid` (`/Game/Mods/SexilesMod/ActorComponents/ac_SXM_Leash.SXM Rope Actor` _returnvalue_2)
            (:`Is Valid`
              (bind _victimactor (`/Game/Mods/SexilesMod/ActorComponents/ac_SXM_Leash.VictimActor` _returnvalue_2))
              (bind _asbase_player_char_2 (cast `/Game/Characters/BasePlayerChar` _victimactor)
                (:`then`
                  (set `self.VictimBasePlayer` _asbase_player_char_2)
                  (bind _asconan_player_controller (cast `ConanPlayerController` (`/Game/Characters/FuncomFunctionLibrary.GetControllerFromActor` _asbase_player_char_2))
                    (:`then`
                      (set `self.VictimController` _asconan_player_controller))
                    (:`CastFailed`
                      _))
                  (`/Game/Mods/SexilesMod/ActorComponents/ac_SXM_Leash.CleanUP` _returnvalue_2)
                  (return true))
                (:`CastFailed`
                  (bind _asbase_npc (cast `/Game/Characters/BaseNPC` _victimactor)
                    (:`then`
                      (set `self.ThrallReference` _asbase_npc)
                      (bind _asbase_player_char_3 (cast `/Game/Characters/BasePlayerChar` _returnvalue)
                        (:`then`
                          (set `self.VictimBasePlayer` _asbase_player_char_3)
                          (set `self.IsThrall` true))
                        (:`CastFailed`
                          _))
                      (`/Game/Mods/SexilesMod/ActorComponents/ac_SXM_Leash.CleanUP` _returnvalue_2)
                      (return false))
                    (:`CastFailed`
                      _)))))
            (:`Is Not Valid`
              _)))
        (:`Is Not Valid`
          _))
      (set `self.VictimController` VictimController)
      (bind _asbase_player_char_4 (cast `/Game/Characters/BasePlayerChar` _returnvalue)
        (:`then`
          (set `self.VictimBasePlayer` _asbase_player_char_4))
        (:`CastFailed`
          _))
      (return true))
    (:`CastFailed`
      (return false))))

(fn `UserConstructionScript`
  (`parent.UserConstructionScript`))