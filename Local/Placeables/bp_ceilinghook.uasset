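; Placeable ceiling hook that toggles a hanging pose on a player or thrall when activated.
; SelectVictim picks the player or NPC held by the instigator's offhand rope, or the instigator when no rope is equipped.
; RCP animation calls move the victim to a helper transform; players switch to Flying.
; A movement-updated callback releases players when velocity changes, while reactivation also releases, returning thralls to their saved transform.
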(event `CustomEvent_0`
  (params (DeltaSeconds :type "Float (double-precision)") (OldLocation :type "Vector Structure") (OldVelocity :type "Vector Structure"))
  (if (not (== OldVelocity (`self.GetVelocity` (`self.VictimController`))))
    ;[1 1 1] Release
    (bind _asbase_player_char (cast `/Game/Characters/BasePlayerChar` (`Controller.K2_GetPawn` (`self.VictimController`)) :!label _label))
    (remove `Character.OnCharacterMovementUpdated` _asbase_player_char (delegate `CustomEvent_0`))
    (`CharacterMovementComponent.SetMovementMode` (`Character.CharacterMovement` _asbase_player_char) "MOVE_Walking" 0)
    (`/Game/Mods/SexilesMod/Character/SXM_BP_PC.RCPPlayAnim` :`self` _asbase_player_char :`Stop` true :`NewAnimToPlay` "/Game/Characters/humans/animations/cinematic/Marketing_Crucifix_Pose_F.Marketing_Crucifix_Pose_F")
    (set `self.ActorInPose` false)
    (set `self.VictimController` null)
    (set `self.VictimBasePlayer` null)))

(event `InteractableInterface.InteractableActivate`
  (params (Component :type "PrimitiveComponent Object Reference") (Instigator :type "PlayerController Object Reference") (HitIndex :type Integer))
  (bind _victimbaseplayer (`self.VictimBasePlayer`))
  (bind _thrallreference (`self.ThrallReference`))
  (if (`self.ActorInPose`)
    (if (`self.IsThrall`)
      (set `self.ActorInPose` false)
      (`/Game/Mods/SexilesMod/Character/SXM_BP_PC.RCPPlayAnim_NPC` (`self.VictimBasePlayer`) true null true (`self.ThrallReference`) (`self.ThrallReturnLocation`))
      (else
        (goto _label)))
    (else
      ;[1 1 1] Set In pose
      (bind _playercharacter (`self.SelectVictim` Instigator))
      (if _playercharacter
        (add `Character.OnCharacterMovementUpdated` _victimbaseplayer (delegate `CustomEvent_0`))
        (`CharacterMovementComponent.SetMovementMode` (`Character.CharacterMovement` _victimbaseplayer) "MOVE_Flying" 0)
        (`KismetSystemLibrary.Delay` 0.2)
        (set `self.ActorInPose` true)
        ;;[1 0.9601 0.217] RCP Function
        (`/Game/Mods/SexilesMod/Character/SXM_BP_PC.RCPPlayAnim` (`self.VictimBasePlayer`) false "/Game/Mods/SexilesMod/Animation_Temp/A_ceiling_hanging.A_ceiling_hanging" true (`SceneComponent.K2_GetComponentToWorld` (`self.PoistionHelper`)) "/Game/Mods/SexilesMod/Character/Anims/Poses/SXM_pose_ceilinghook.SXM_pose_ceilinghook")
        (else
          (set `self.ActorInPose` true)
          (set `self.ThrallReturnLocation` (`self.GetTransform` _thrallreference))
          (`/Game/Mods/SexilesMod/Character/SXM_BP_PC.RCPPlayAnim_NPC` (`self.VictimBasePlayer`) false "/Game/Mods/SexilesMod/Animation_Temp/A_ceiling_hanging.A_ceiling_hanging" true _thrallreference (`SceneComponent.K2_GetComponentToWorld` (`self.PoistionHelper`))))))))

(fn `SelectVictim`
  (params (VictimController :type "PlayerController Object Reference"))
  (returns (PlayerCharacter :type Boolean))
  (bind _returnvalue (`Controller.K2_GetPawn` VictimController))
  (bind _asbase_player_char (cast `/Game/Characters/BasePlayerChar` (`Controller.K2_GetPawn` VictimController))
    (:`then`
      (bind _asbp_rope_1h_new (cast `/Game/Mods/SexilesMod/Weapons/BP_rope_1h_new` (`GameItem.VisualActor` (`/Game/Characters/BaseBPCombat.GetOffhandWeapon` _asbase_player_char)))
        (:`then`
          (bind _victimactor (`/Game/Mods/SexilesMod/Weapons/BP_rope_1h_new.victimactor` _asbp_rope_1h_new))
          (bind _asbase_player_char_2 (cast `/Game/Characters/BasePlayerChar` _victimactor)
            (:`then`
              (set `self.VictimBasePlayer` _asbase_player_char_2)
              (bind _asconan_player_controller (cast `ConanPlayerController` (`/Game/Characters/FuncomFunctionLibrary.GetControllerFromActor` _asbase_player_char_2))
                (:`then`
                  (set `self.VictimController` _asconan_player_controller)
                  (return true))
                (:`CastFailed`
                  _)))
            (:`CastFailed`
              (bind _asbase_npc (cast `/Game/Characters/BaseNPC` _victimactor)
                (:`then`
                  (set `self.ThrallReference` _asbase_npc)
                  (bind _asbase_player_char_3 (cast `/Game/Characters/BasePlayerChar` _returnvalue)
                    (:`then`
                      (set `self.VictimBasePlayer` _asbase_player_char_3)
                      (set `self.IsThrall` true))
                    (:`CastFailed`
                      _)))
                (:`CastFailed`
                  (set `self.VictimController` VictimController :!label _label)
                  (bind _asbase_player_char_4 (cast `/Game/Characters/BasePlayerChar` _returnvalue)
                    (:`then`
                      (set `self.VictimBasePlayer` _asbase_player_char_4)
                      (return true))
                    (:`CastFailed`
                      _)))))))
        (:`CastFailed`
          (goto _label)))
      (return false))
    (:`CastFailed`
      (return false))))

(fn `UserConstructionScript`
  (`parent.UserConstructionScript`))