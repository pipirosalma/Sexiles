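; Placeable ceiling chains that pose a player, either the one interacting or the player on their SXM leash, at the sit point.
; Activation picks the victim, clears any leashed victim, transforms and animates the character, and spawns a chain-material rope actor.
; Re-activating releases a player to walking, as does a velocity mismatch in the bound movement-update event.
; Leashed NPCs are recorded but not posed, and most cable-attachment experiments are disconnected.
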(event `CustomEvent_0`
  (params (DeltaSeconds :type "Float (double-precision)") (OldLocation :type "Vector Structure") (OldVelocity :type "Vector Structure"))
  (if (not (== OldVelocity (`self.GetVelocity` (`self.VictimController`))))
    ;[1 1 1] Release
    (bind _asbase_player_char (cast `/Game/Characters/BasePlayerChar` (`Controller.K2_GetPawn` (`self.VictimController`)) :!label _label))
    (remove `Character.OnCharacterMovementUpdated` _asbase_player_char (delegate `CustomEvent_0`))
    (`CharacterMovementComponent.SetMovementMode` (`Character.CharacterMovement` _asbase_player_char) "MOVE_Walking" 0)
    (`/Game/Mods/SexilesMod/Character/SXM_BP_PC.RCPPlayAnim` :`self` _asbase_player_char :`Stop` true :`NewAnimToPlay` "/Game/Characters/humans/animations/cinematic/Marketing_Crucifix_Pose_F.Marketing_Crucifix_Pose_F")
    (set `self.ActorInPose` false)
    (set `self.VictimController` null)
    (set `self.VictimBasePlayer` null)))

(event `InteractableInterface.InteractableActivate`
  (params (Component :type "PrimitiveComponent Object Reference") (Instigator :type "PlayerController Object Reference") (HitIndex :type Integer))
  (bind _victimbaseplayer (`self.VictimBasePlayer`))
  (bind _victimbaseplayer_2 (`self.VictimBasePlayer`))
  (bind _victimbaseplayer_3 (`self.VictimBasePlayer`))
  (bind _returnvalue (`SceneComponent.K2_GetComponentToWorld` (`self.BP_BSC_Sit`)))
  (if (`self.ActorInPose`)
    (if (`self.IsThrall`)
      (set `self.ActorInPose` false)
      (else
        (goto _label)))
    (else
      ;[1 1 1] Set In pose
      (bind _playercharacter (`self.Select Victim` Instigator))
      (if _playercharacter
        (add `Character.OnCharacterMovementUpdated` _victimbaseplayer (delegate `CustomEvent_0`))
        (set `self.ActorInPose` true)
        ;;[1 0.9601 0.217] RCP Function
        (`/Game/Mods/SexilesMod/Character/SXM_BP_PC.TransformActor` _victimbaseplayer_3 _returnvalue (`KismetMathLibrary.MakeTransform` (`KismetMathLibrary.MakeVector` (.x (.location _returnvalue)) (.y (.location _returnvalue)) (.z (.location (`SceneComponent.K2_GetComponentToWorld` (`Character.CapsuleComponent` _victimbaseplayer))))) (.rotation _returnvalue) (.scale _returnvalue)))
        (`/Game/Mods/SexilesMod/Character/SXM_BP_PC.Activate` _victimbaseplayer_3 12 false)
        (`|SpawnActorFromClass` "/Game/Mods/SexilesMod/System/SXM_RopeActor.SXM_RopeActor_C" (`self.GetTransform` _victimbaseplayer_2) "Undefined" "OverrideRootScale" self _victimbaseplayer_2 "/Game/Items/Weapons/Lasso/Materials/M_chains_lasso.M_chains_lasso")))))

(event `SetChains`
  (params (Condition :type Boolean))
  (if Condition
    (`CableComponent.SetAttachEndTo` (`self.Cable`) (`self.VictimBasePlayer`) "None" "b_L_hand")))

(fn `Select Victim`
  (params (InputPin :type "PlayerController Object Reference"))
  (returns (PlayerCharacter :type Boolean))
  (bind _returnvalue (`Controller.K2_GetPawn` InputPin))
  (bind _asbase_player_char (cast `/Game/Characters/BasePlayerChar` (`Controller.K2_GetPawn` InputPin))
    (:`then`
      (bind _returnvalue_2 (`self.GetComponentByClass` _asbase_player_char "/Game/Mods/SexilesMod/ActorComponents/ac_SXM_Leash.ac_SXM_Leash_C"))
      (`/Engine/EditorBlueprintResources/StandardMacros.IsValid` _returnvalue_2
        (:`Is Valid`
          (`/Engine/EditorBlueprintResources/StandardMacros.IsValid` (`/Game/Mods/SexilesMod/ActorComponents/ac_SXM_Leash.SXM Rope Actor` _returnvalue_2)
            (:`Is Valid`
              (bind _victimactor (`/Game/Mods/SexilesMod/ActorComponents/ac_SXM_Leash.VictimActor` _returnvalue_2))
              (bind _asbase_player_char_2 (cast `/Game/Characters/BasePlayerChar` _victimactor)
                (:`then`
                  (set `self.VictimBasePlayer` _asbase_player_char_2)
                  (bind _asconan_player_controller (cast `ConanPlayerController` (`/Game/Characters/FuncomFunctionLibrary.GetControllerFromActor` _asbase_player_char_2))
                    (:`then`
                      (set `self.VictimController` _asconan_player_controller))
                    (:`CastFailed`
                      _))
                  (`/Game/Mods/SexilesMod/ActorComponents/ac_SXM_Leash.CleanUP` _returnvalue_2)
                  (return true))
                (:`CastFailed`
                  (bind _asbase_npc (cast `/Game/Characters/BaseNPC` _victimactor)
                    (:`then`
                      (set `self.ThrallReference` _asbase_npc)
                      (bind _asbase_player_char_3 (cast `/Game/Characters/BasePlayerChar` _returnvalue)
                        (:`then`
                          (set `self.VictimBasePlayer` _asbase_player_char_3)
                          (set `self.IsThrall` true))
                        (:`CastFailed`
                          _))
                      (`/Game/Mods/SexilesMod/ActorComponents/ac_SXM_Leash.CleanUP` _returnvalue_2)
                      (return false))
                    (:`CastFailed`
                      _)))))
            (:`Is Not Valid`
              _)))
        (:`Is Not Valid`
          _))
      (set `self.VictimController` InputPin)
      (bind _asbase_player_char_4 (cast `/Game/Characters/BasePlayerChar` _returnvalue)
        (:`then`
          (set `self.VictimBasePlayer` _asbase_player_char_4))
        (:`CastFailed`
          _))
      (return true))
    (:`CastFailed`
      (return false))))

(fn `UserConstructionScript`
  (`parent.UserConstructionScript`))