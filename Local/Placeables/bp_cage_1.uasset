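; Placeable cage whose door swings open and shut when a player interacts with it.
; Interaction requires a specific item in the player's backpack or ownership of the cage, then plays or reverses a timeline that yaws the door mesh up to 90 degrees.
; Victim posing via SelectVictim, which prefers a rope-held captive, is present but disconnected, along with its movement-update handler that releases the victim on velocity change.
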(event `CustomEvent_0`
  (params (DeltaSeconds :type "Float (double-precision)") (OldLocation :type "Vector Structure") (OldVelocity :type "Vector Structure"))
  (if (not (== OldVelocity (`self.GetVelocity` (`self.VictimController`)) :`ErrorTolerance` 0.01))
    ;[1 1 1] Release
    (bind _asbase_player_char (cast `/Game/Characters/BasePlayerChar` (`Controller.K2_GetPawn` (`self.VictimController`))))
    (remove `Character.OnCharacterMovementUpdated` _asbase_player_char (delegate `CustomEvent_0`))
    (set `self.ActorInPose` false)
    (set `self.VictimController` null)
    (set `self.VictimBasePlayer` null)))

(event `InteractableInterface.InteractableActivate`
  (params (Component :type "PrimitiveComponent Object Reference") (Instigator :type "PlayerController Object Reference") (HitIndex :type Integer))
  (bind _returnvalue (`Controller.K2_GetPawn` Instigator))
  (bind _sm_cagedoor (`self.SM_CageDoor`))
  (bind _asbase_player_char (cast `/Game/Characters/BasePlayerChar` _returnvalue))
  (bind _returnvalue_2 (`ConanCharacter.GetBackpackInventory` _asbase_player_char))
  (if (`ItemInventory.HasItemByTemplateID` _returnvalue_2 295507 1)
    (if (`self.IsOpen`) :!label _label
      (bind (_direction _rotation) (`Timeline|OpenDoor` :!label _label_2)
        (:`Update`
          (`self.RotateDoor` _sm_cagedoor (`KismetMathLibrary.MakeRotator` (.roll (`SceneComponent.RelativeRotation` _sm_cagedoor)) (.pitch (`SceneComponent.RelativeRotation` _sm_cagedoor)) (* _rotation 90.0))))
        (:`Finished`
          (set `self.IsOpen` (not (`self.IsOpen`)))))
      (else
        (goto _label_2 :!via `Reverse`)))
    (elif (`self.IsOwner` _returnvalue true)
      (goto _label))))

(event `RotateDoor`
  (params (Target :type "SceneComponent Object Reference") (NewRotation :type "Rotator Structure"))
  (`SceneComponent.K2_SetRelativeRotation` Target NewRotation false false))

(fn `SelectVictim`
  (params (VictimController :type "PlayerController Object Reference"))
  (bind _asbase_player_char (cast `/Game/Characters/BasePlayerChar` (`Controller.K2_GetPawn` VictimController)))
  (bind _asbp_rope_1h_new (cast `/Game/Mods/SexilesMod/Weapons/BP_rope_1h_new` (`GameItem.VisualActor` (`/Game/Characters/BaseBPCombat.GetOffhandWeapon` _asbase_player_char)))
    (:`then`
      (bind _asbase_player_char_2 (cast `/Game/Characters/BasePlayerChar` (`/Game/Mods/SexilesMod/Weapons/BP_rope_1h_new.victimactor` _asbp_rope_1h_new))
        (:`then`
          (set `self.VictimBasePlayer` _asbase_player_char_2)
          (bind _asconan_player_controller (cast `ConanPlayerController` (`/Game/Characters/FuncomFunctionLibrary.GetControllerFromActor` _asbase_player_char_2)))
          (set `self.VictimController` _asconan_player_controller))
        (:`CastFailed`
          (set `self.VictimController` VictimController :!label _label)
          (bind _asbase_player_char_3 (cast `/Game/Characters/BasePlayerChar` (`Controller.K2_GetPawn` VictimController)))
          (set `self.VictimBasePlayer` _asbase_player_char_3))))
    (:`CastFailed`
      (goto _label))))

(fn `UserConstructionScript`
  (`parent.UserConstructionScript`))