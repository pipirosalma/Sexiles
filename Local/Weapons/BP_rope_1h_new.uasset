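; One-handed rope weapon that leashes a collared player or NPC to its wielder, attaching a cable to the victim's neck socket.
; Tick measures the distance: straying players get suffocation or break warnings, and unconscious ones are dragged along.
; NPCs follow through AIMoveTo, updating their thrall home location.
; The rope force-unequips when the collar is gone or a conscious player or NPC gets too far away.
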(event `self.ReceiveTick`
  (params (DeltaSeconds :type "Float (single-precision)"))
  (bind _returnvalue (`self.GetOwner`))
  (bind _victimactor (`self.victimactor`))
  (bind _victimactor_2 (`self.victimactor`))
  (bind _victimactor_3 (`self.victimactor`))
  (bind _returnvalue_2 (`self.K2_GetActorLocation` _returnvalue))
  (bind _returnvalue_3 (- (`self.K2_GetActorLocation` (`self.GetOwner`)) (`self.K2_GetActorLocation` (`self.victimactor`))))
  (bind _returnvalue_4 (`KismetMathLibrary.VSize` (- (`self.K2_GetActorLocation` _victimactor) _returnvalue_2)))
  (bind _returnvalue_5 (> _returnvalue_4 2000.0))
  (`/Engine/EditorBlueprintResources/StandardMacros.IsValid` _victimactor_2
    (:`Is Valid`
      (bind _collared (`self.CollarCheck` _victimactor_2)
        (:`Completed`
          (if _collared
            (bind _asbase_player_char (cast `/Game/Characters/BasePlayerChar` _victimactor)
              (:`then`
                (bind _asfun_combat_player_controller (cast `/Game/Systems/FunCombat_PlayerController` (`/Game/Characters/FuncomFunctionLibrary.GetControllerFromActor` (`self.GetOwner`))))
                (if (> _returnvalue_4 700.0)
                  (if (`|EnumInequality` (`ConanCharacter.GetCharacterState` _asbase_player_char) "Unconscious")
                    (if _returnvalue_5
                      (`GameItem.ForceUnequip` (`self.GetOwnerWeaponItem`) :!label _label)
                      (elif (> _returnvalue_4 1300.0)
                        (`/Game/Systems/FunCombat_PlayerController.NotificationText` _asfun_combat_player_controller "The tope will Brake soon!" false)
                        (else
                          ;[1 1 1] suffocation %
                          (`/Game/Systems/FunCombat_PlayerController.NotificationText` _asfun_combat_player_controller "The rope suffocates your victim!" false)
                          (bind _00_bp_ac_buffsystem (`/Game/Characters/BaseBPCombat.00_BP_AC_BuffSystem` _asbase_player_char))
                          (`/Game/Systems/Buffs/00_BP_AC_BuffSystem.AddBuff` _00_bp_ac_buffsystem "/Game/Mods/SexilesMod/System/00_BP_AC_Sufocation.00_BP_AC_Sufocation_C" null 0 null))))
                    (else
                      (`self.K2_SetActorLocation` _victimactor_3 (+ (`self.K2_GetActorLocation` _victimactor_3) (* _returnvalue_3 (/ (- (`KismetMathLibrary.VSize` _returnvalue_3) 500.0) 1000.0))) false false)))
                  (elif (> _returnvalue_4 200.0)
                    (if (`/Game/Systems/Buffs/00_BP_AC_BuffSystem.CheckIfBuffExists` _00_bp_ac_buffsystem "/Game/Mods/SexilesMod/System/00_BP_AC_Sufocation.00_BP_AC_Sufocation_C")
                      (`/Game/Systems/Buffs/00_BP_AC_BuffSystem.EndBuff` _00_bp_ac_buffsystem "/Game/Mods/SexilesMod/System/00_BP_AC_Sufocation.00_BP_AC_Sufocation_C")))))
              (:`CastFailed`
                (if _returnvalue_5
                  (goto _label)
                  (else
                    (bind _asbase_npc (cast `/Game/Characters/BaseNPC` _victimactor))
                    (`|AIMoveTo` _asbase_npc _asbase_npc _returnvalue_2 _returnvalue 200.0
                      (:`then`
                        (`ThrallComponent.UpdateHomeLocation` (`self.GetComponentByClass` _asbase_npc "/Game/Systems/Thrall/BP_ThrallComponent.BP_ThrallComponent_C") _returnvalue_2)))))))
            (else
              (`GameItem.ForceUnequip` (`self.GetOwnerWeaponItem`) :!label _label_2))))))))

(event `RopeUnequip`
  (goto _label_2))

(event `MakeRopeConnection`
  (params (InputPin :type "/Game/Characters/BaseBPChar Object Reference"))
  (bind _output_get (set `self.victimactor` InputPin :!label _label_3))
  (bind _collared (`self.CollarCheck` _output_get)
    (:`Completed`
      (if _collared
        (`self.RopeConnect` InputPin _output_get)
        (bind _asbase_player_char (cast `/Game/Characters/BasePlayerChar` InputPin))
        (`/Game/Mods/SexilesMod/Character/SXM_BP_PC.SetBoundObject` _asbase_player_char false (0.0 0.0 0.0) null)
        (else
          (`SceneComponent.K2_DetachFromComponent` (`self.Cable`) "KeepRelative" "KeepRelative" "KeepRelative" true :!label _label_4)
          (set `self.victimactor` null))))))

(event `self.ReceiveBeginPlay`
  (cast `/Local/Weapons/BP_rope_1h_new` (`GameItem.VisualActor` (`/Game/Characters/BaseBPCombat.GetOffhandWeapon` (`self.GetBasePlayerChar`)))
    (:`then`
      (goto _label_3))
    (:`CastFailed`
      (`/Engine/EditorBlueprintResources/StandardMacros.IsValid` (`self.Cable`)
        (:`Is Valid`
          (goto _label_4))))))

(event `destroyrope`
  (bind _asbase_player_char (cast `/Game/Characters/BasePlayerChar` (`self.victimactor`))
    (:`then`
      (bind _00_bp_ac_buffsystem (`/Game/Characters/BaseBPCombat.00_BP_AC_BuffSystem` _asbase_player_char))
      (if (`/Game/Systems/Buffs/00_BP_AC_BuffSystem.CheckIfBuffExists` _00_bp_ac_buffsystem "/Game/Mods/SexilesMod/System/00_BP_AC_Sufocation.00_BP_AC_Sufocation_C")
        (`/Game/Systems/Buffs/00_BP_AC_BuffSystem.EndBuff` _00_bp_ac_buffsystem "/Game/Mods/SexilesMod/System/00_BP_AC_Sufocation.00_BP_AC_Sufocation_C")))
    (:`CastFailed`
      _))
  (`SceneComponent.K2_DetachFromComponent` (`self.Cable`) "KeepRelative" "KeepRelative" "KeepRelative" true))

(fn `CastTrace`
  (returns (`AsBase BPChar` :type "/Game/Characters/BaseBPChar Object Reference"))
  (bind _aspawn (cast `Pawn` (`self.GetOwner`))
    (:`then`
      (bind (_outputpin _output_get) (`self.NewMacro_0` (`self.GetBasePlayerChar`)))
      (bind _outhit (`KismetSystemLibrary.SphereTraceSingleForObjects` _outputpin _output_get 130.0 (`|MakeArray` "ObjectTypeQuery3" :!type "EObjectTypeQuery Enum") false (`|MakeArray` _aspawn :!type "Actor Object Reference") "ForDuration"))
      (bind _asbase_bpchar (cast `/Game/Characters/BaseBPChar` (`.HitActor` (`GameplayStatics.BreakHitResult` _outhit)))
        (:`then`
          _)
        (:`CastFailed`
          _)))
    (:`CastFailed`
      _))
  (return _asbase_bpchar))

(fn `GetBasePlayerChar`
  (returns (BasePlayerChar :type "/Game/Characters/BasePlayerChar Object Reference"))
  (bind _returnvalue (`self.GetOwner`))
  (bind _asfun_combat_player_controller (cast `/Game/Systems/FunCombat_PlayerController` _returnvalue)
    (:`then`
      (cast `/Game/Characters/BasePlayerChar` (`Controller.K2_GetPawn` _asfun_combat_player_controller)
        (:`then`
          _)
        (:`CastFailed`
          _)))
    (:`CastFailed`
      (bind _asbase_player_char (cast `/Game/Characters/BasePlayerChar` _returnvalue)
        (:`then`
          _)
        (:`CastFailed`
          _))))
  (return _asbase_player_char))

(fn `RopeConnect`
  (params (BasePlayerChar :type "/Game/Characters/BaseBPChar Object Reference") (Target :type "Actor Object Reference"))
  (locals (NewLocalVar_0 :type Boolean))
  (`SceneComponent.K2_AttachToComponent` (`self.Cable`) (`KismetArrayLibrary.Array_Get` (`self.K2_GetComponentsByClass` Target "/Script/Engine.SkeletalMeshComponent")) "b_neck_2" "SnapToTarget" "SnapToTarget" "SnapToTarget" true))

(fn `UserConstructionScript`
  (`parent.UserConstructionScript`))