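; Actor component that lets a player character leash a victim actor with a visible rope.
; Making a connection toggles: it destroys an existing rope actor, otherwise spawns an SXM_RopeActor attached to the victim's neck socket and linked to the player.
; The rope material follows the offhand item's template ID, defaulting to the basic lasso.
; A weapon-equipped signal removes the rope when the offhand visual is no longer the one-handed rope.
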(event `self.ReceiveBeginPlay`
  ;[0.2891 1 0.3467] BeginPlay and Event  Binds
  (add `/Game/Characters/BaseBPCombat.SignalWeaponEquipped` (`self.GetBasePlayerCharacter`) (delegate `SignalWeaponEquipped_Event_0`)))

(event `MakeRopeConnection`
  (params (VictimActor :type "/Game/Characters/BaseBPCombat Object Reference"))
  ;[0.3833 0.4599 1] Create Rope Connection
  (`/Engine/EditorBlueprintResources/StandardMacros.IsValid` (`self.SXM Rope Actor`)
    (:`Is Valid`
      (`self.CleanUP`))
    (:`Is Not Valid`
      (`self.MakeRopeConnection_C` VictimActor))))

(event `CleanUP`
  ;[0.3833 0.4599 1] Create Rope Connection
  ;;[1 0.8976 0] CleanUp
  (`Actor.K2_DestroyActor` (`self.SXM Rope Actor`))
  (set `self.VictimActor` null))

(event `SignalWeaponEquipped_Event_0`
  (params (Item :type "GameItem Object Reference"))
  ;[0.2891 1 0.3467] BeginPlay and Event  Binds
  (bind _returnvalue (`GameItem.GetVisualObjectClass` (`/Game/Characters/BaseBPCombat.GetOffhandWeapon` (`self.GetBasePlayerCharacter`))))
  (if (not (== _returnvalue "/Game/Items/Weapons/Rope/BP_rope_1h.BP_rope_1h_C"))
    (`/Engine/EditorBlueprintResources/StandardMacros.IsValid` (`self.SXM Rope Actor`)
      (:`Is Valid`
        (`self.CleanUP`)))))

(event `MakeRopeConnection_C`
  (params (VictimActor :type "/Game/Characters/BaseBPCombat Object Reference"))
  ;[0.3833 0.4599 1] Create Rope Connection
  (set `self.VictimActor` VictimActor)
  (bind _value (`self.GetRopeMaterial`)
    (:`OutputPin`
      (bind _returnvalue (`|SpawnActorFromClass` "/Game/Mods/SexilesMod/System/SXM_RopeActor.SXM_RopeActor_C" (`Actor.GetTransform` VictimActor) "Undefined" "OverrideRootScale" VictimActor (`self.GetBasePlayerCharacter`) _value))
      (bind _output_get (set `self.SXM Rope Actor` _returnvalue))
      (`Actor.K2_AttachToComponent` _output_get (`KismetArrayLibrary.Array_Get` (`Actor.K2_GetComponentsByClass` VictimActor "/Script/Engine.SkeletalMeshComponent")) "b_Neck_2" "SnapToTarget" "SnapToTarget" "SnapToTarget" true))))

(fn `GetBasePlayerCharacter`
  (returns (`AsBase Player Char` :type "/Game/Characters/BasePlayerChar Object Reference"))
  (bind _asbase_player_char (cast `/Game/Characters/BasePlayerChar` (`self.GetOwner`)))
  (return _asbase_player_char))

(fn `OnRep_LeashCableComp`)