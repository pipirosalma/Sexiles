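; Player component for the SXM mod that adds a custom radial menu for interacting with humanoid NPCs and thralls.
; When MainRadialMenu opens on a selected NPC, SXM_MainRadialMenu is built from both characters' states.
; Selections route by category to server-relayed emotes, handcuff stages, leashing or paired seduce animations.
; BeginPlay also teaches emotes, resets out-of-range warpaint and hooks a substate-triggered animation; older inline menu-building graphs remain unconnected.
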(event `MainRadialOpen`
  (params (module :type "GUIModule Object Reference") (isActive :type Boolean))
  ;[1 1 1] Bind to MainRadialMenu opening
  (`self.OpenThrallRadialMenu` module isActive))

(event `self.ReceiveBeginPlay`
  (`|ExecutionSequence`
    (:`then_0`
      ;[1 1 1] Bind to MainRadialMenu opening
      (bind _returnvalue (`GUIModuleController.GetModule` (`GUIModuleController.GetGUIModuleController`) "MainRadialMenu"))
      (add `GUIModule.SignalActivated` _returnvalue (delegate `MainRadialOpen`)))
    (:`then_1`
      (bind _asbase_player_char (cast `/Game/Characters/BasePlayerChar` (`self.GetOwner`)))
      (add `/Game/Characters/BaseBPChar.OnCharacterSubstateChanged` _asbase_player_char (delegate `OnCharacterSubstateChanged_Event_0`)))
    (:`then_2`
      (`self.NewMacro_0`))
    (:`then_3`
      (`|ExecutionSequence`
        (:`then_0`
          ;[1 1 1] Bind custom radian menus
          (bind _returnvalue_2 (`GUIModuleController.GetModule` (`GUIModuleController.GetGUIModuleController`) "MainRadialMenu"))
          (add `GUIModule.SignalActivated` _returnvalue_2 (delegate `CallSXM_PC`)))
        (:`then_1`
          ;[1 1 1] Learn new emotes
          (bind _assxm_bp_pc (cast `/Game/Mods/SexilesMod/Character/SXM_BP_PC` (`self.GetOwner`)))
          (`/Game/Mods/SexilesMod/Character/SXM_BP_PC.EmoteLearn` _assxm_bp_pc))))))

(event `ActivateAnimation`
  (params (menuEntry :type "RadialMenuEntry Object Reference"))
  (bind _assxm_bp_pc (cast `/Game/Mods/SexilesMod/Character/SXM_BP_PC` (`self.GetOwner`)))
  (`/Game/Mods/SexilesMod/Character/SXM_BP_PC.SXM_NPCInteraction handle` _assxm_bp_pc true (`RadialMenuEntry.UserValue` menuEntry) (`Actor.GetComponentByClass` (`self.TargetNPC`) "/Game/Mods/SexilesMod/Character/SXM_Component.SXM_Component_C"))
  (`KismetSystemLibrary.Delay` 0.2 :!label _label)
  (`GUIModuleController.ActivateModule` (`GUIModuleController.GetGUIModuleController`) "MainRadialMenu" false false))

(event `OnCharacterSubstateChanged_Event_0`
  (params (Substate :type "/Game/Characters/CharacterSubState Enum") (Entered :type Boolean))
  (`/Game/Systems/BP_MacroGlobal.And+Branch` (`|EnumEquality` Substate "NewEnumerator5") Entered
    (:`True`
      (bind _newparam (`/Game/Characters/BaseBPCombat.GetCurrentEmote` (stale `self.ReceiveBeginPlay` _asbase_player_char)))
      (if (`|EnumEquality` _newparam "Pissing")
        (bind _assxm_bp_pc (cast `/Game/Mods/SexilesMod/Character/SXM_BP_PC` (`self.GetOwner`)))
        (message `/Game/Master_AnimBP/ab_human_male_interface.StopEmoteAnimation` _assxm_bp_pc)
        (`/Game/Characters/BaseBPChar.ExitSubstate` _assxm_bp_pc "NewEnumerator5")
        (`/Game/Mods/SexilesMod/Character/SXM_BP_PC.Activate` _assxm_bp_pc 11 false)))))

(event `PassiveAnimation`
  (params (menuEntry :type "RadialMenuEntry Object Reference"))
  (bind _assxm_bp_pc (cast `/Game/Mods/SexilesMod/Character/SXM_BP_PC` (`self.GetOwner`)))
  (`/Engine/EditorBlueprintResources/StandardMacros.IsValid` (`self.TargetNPC`)
    (:`Is Valid`
      (`/Game/Mods/SexilesMod/Character/SXM_BP_PC.SXM_NPCInteraction handle` _assxm_bp_pc false (`RadialMenuEntry.UserValue` menuEntry) (`Actor.GetComponentByClass` (`self.TargetNPC`) "/Game/Mods/SexilesMod/Character/SXM_Component.SXM_Component_C"))
      (goto _label))
    (:`Is Not Valid`
      (`KismetSystemLibrary.PrintString` "nope"))))

(event `TieLeashSelected`
  (params (menuEntry :type "RadialMenuEntry Object Reference"))
  (`/Game/Mods/SexilesMod/ActorComponents/ac_SXM_Leash.MakeRopeConnection` (`Actor.GetComponentByClass` (`self.GetOwner`) "/Game/Mods/SexilesMod/ActorComponents/ac_SXM_Leash.ac_SXM_Leash_C") (`self.TargetNPC`)))

(event `Emote Selected`
  (params (menuEntry :type "RadialMenuEntry Object Reference"))
  (`self.ChangeThrallValues` true (`Actor.GetComponentByClass` (`self.TargetNPC`) "/Game/Mods/SexilesMod/ActorComponents/SXM_AC_NPC.SXM_AC_NPC_C") (`KismetStringLibrary.Conv_StringToName` (`KismetStringLibrary.Conv_IntToString` (`RadialMenuEntry.UserValue` menuEntry))) "Aggressive")
  (`GUIModuleController.ActivateModule` (`GUIModuleController.GetGUIModuleController`) "MainRadialMenu" false false))

(event `CallSXM_PC`
  (params (module :type "GUIModule Object Reference") (isActive :type Boolean))
  ;[1 1 1] Bind custom radian menus
  (bind _assxm_bp_pc (cast `/Game/Mods/SexilesMod/Character/SXM_BP_PC` (`self.GetOwner`)))
  (`/Game/Mods/SexilesMod/Character/SXM_BP_PC.CustomRadialsHandle` _assxm_bp_pc module isActive))

(event `ChangeAgression`
  (params (menuEntry :type "RadialMenuEntry Object Reference"))
  (bind _returnvalue (`Actor.GetComponentByClass` (`self.TargetNPC`) "/Game/Mods/SexilesMod/ActorComponents/SXM_AC_NPC.SXM_AC_NPC_C"))
  (if (`|EnumEquality` (`/Game/Mods/SexilesMod/ActorComponents/SXM_AC_NPC.AggroState` (`Actor.GetComponentByClass` (`self.TargetNPC`) "/Game/Mods/SexilesMod/ActorComponents/SXM_AC_NPC.SXM_AC_NPC_C")) "Aggressive")
    (`self.ChangeThrallValues` false _returnvalue "None" "Aggressive")
    (else
      (`self.ChangeThrallValues` false _returnvalue "None" "Passive"))))

(event `UnlockHands`
  (params (menuEntry :type "RadialMenuEntry Object Reference"))
  (bind _asbase_player_char (cast `/Game/Characters/BasePlayerChar` (`self.GetOwner`)))
  (`/Game/Mods/SexilesMod/Character/SXM_Component.SetLockStage` (`Actor.GetComponentByClass` _asbase_player_char "/Game/Mods/SexilesMod/Character/SXM_Component.SXM_Component_C") 2))

(event `OpenThrallRadialMenu`
  (params (module :type "GUIModule Object Reference") (isActive :type Boolean))
  (bind _targetnpc (`self.TargetNPC`))
  ;[1 1 1] Open radial menu for Thralls
  (if isActive
    (bind _asfun_combat_player_controller (cast `/Game/Systems/FunCombat_PlayerController` (`/Game/Characters/FuncomFunctionLibrary.GetControllerFromActor` (`self.GetOwner`))))
    (bind _returnvalue (`/Game/Systems/FunCombat_PlayerController.GetInteractionManager` _asfun_combat_player_controller))
    (if (`/Game/Systems/InteractionManager.HasSelectedObject` _returnvalue)
      (bind _aspersistent_humanoid_npc (cast `/Game/Characters/NPCs/Humanoid/PersistentHumanoidNPC` (`KismetSystemLibrary.Conv_InterfaceToObject` (`/Game/Systems/InteractionManager.SelectedObject` _returnvalue))))
      (set `self.TargetNPC` _aspersistent_humanoid_npc)
      ;[1 1 1] Build the menu
      (bind (_guimodule _windowroot) (`GUIModule_Activate_CallProxy.GUIModule_Activate` module true)
        (:`OnActivate`
          (bind _asw_main_radial_menu (cast `/Game/UI/RadialMenus/W_MainRadialMenu` _windowroot))
          (bind (_module _windowroot_2) (`GUIModuleController_Activate_CallProxy.GUIModuleController_Activate` (`GUIModuleController.GetGUIModuleController`) "SXM_MainRadialMenu" true)
            (:`OnActivate`
              (bind _asw_sxm_main_radial_menu (cast `/Game/Mods/SexilesMod/UI/W_SXM_MainRadialMenu` _windowroot_2))
              (bind _asbase_bpcombat (cast `/Game/Characters/BaseBPCombat` (`self.GetOwner`)))
              (bind _state (`/Game/Mods/SexilesMod/Character/SXM_Library.SXML_GetCharacterState` _asbase_bpcombat _targetnpc))
              (bind _state_2 (`/Game/Mods/SexilesMod/Character/SXM_Library.SXML_GetCharacterState` _targetnpc))
              (`/Game/Mods/SexilesMod/UI/W_SXM_MainRadialMenu.BuildMenuThrall` _asw_sxm_main_radial_menu _state _state_2 _asw_main_radial_menu)
              (add `/Game/Mods/SexilesMod/UI/W_SXM_MainRadialMenu.MenuItemSelected` _asw_sxm_main_radial_menu (delegate `OnThrallMenuSelected`)))))))))

(event `ChangeThrallValues`
  (params (Emote :type Boolean) (Target :type "/Game/Mods/SexilesMod/ActorComponents/SXM_AC_NPC Object Reference") (EmoteToPlay :type Name) (AggroState :type "ECharacterState Enum"))
  ;[1 1 1] SERVER - Handle menu options
  (`self.ChangeThrallValues_SRV` Emote Target EmoteToPlay AggroState))

(event `ChangeThrallValues_SRV`
  (params (Emote :type Boolean) (Target :type "/Game/Mods/SexilesMod/ActorComponents/SXM_AC_NPC Object Reference") (EmoteToPlay :type Name) (AggroState :type "ECharacterState Enum"))
  ;[1 1 1] SERVER - Handle menu options
  (`self.ChangeThrallValues_C` Emote Target EmoteToPlay AggroState))

(event `ChangeThrallValues_C`
  (params (Emote :type Boolean) (Target :type "/Game/Mods/SexilesMod/ActorComponents/SXM_AC_NPC Object Reference") (EmoteToPlay :type Name) (AggroState :type "ECharacterState Enum"))
  ;[1 1 1] SERVER - Handle menu options
  (if Emote
    (`/Game/Mods/SexilesMod/ActorComponents/SXM_AC_NPC.SetNewEmote` Target EmoteToPlay)))

(event `OnThrallMenuSelected`
  (params (RowName :type Name) (CategoryID :type "/Game/Mods/SexilesMod/Types/SXM_MenuCategory Enum") (AnimationIndex :type Integer) (PlayerState :type "/Game/Mods/SexilesMod/Types/S_SXM_CharacterState Structure") (TargetState :type "/Game/Mods/SexilesMod/Types/S_SXM_CharacterState Structure"))
  ;[1 1 1] Handle menu select
  (set `self.MenuSelectedAnimationIndex` AnimationIndex)
  (`GUIModule_Activate_CallProxy.GUIModule_Activate` (stale `OpenThrallRadialMenu` _guimodule) false true
    (:`then`
      (switch `/Game/Mods/SexilesMod/Types/SXM_MenuCategory` CategoryID
        (:`NewEnumerator1`
          ;[1 1 1] Play Emote
          (`self.ChangeThrallValues` true (`Actor.GetComponentByClass` (`self.TargetNPC`) "/Game/Mods/SexilesMod/ActorComponents/SXM_AC_NPC.SXM_AC_NPC_C") (`KismetStringLibrary.Conv_StringToName` (`KismetStringLibrary.Conv_IntToString` (`self.MenuSelectedAnimationIndex`))) "Aggressive"))
        (:`NewEnumerator5`
          ;[1 1 1] Unlock cuffs
          (bind _asbase_player_char (cast `/Game/Characters/BasePlayerChar` (`self.GetOwner`)))
          (`/Game/Mods/SexilesMod/Character/SXM_Component.SetLockStage` (`Actor.GetComponentByClass` _asbase_player_char "/Game/Mods/SexilesMod/Character/SXM_Component.SXM_Component_C") (`self.MenuSelectedAnimationIndex`)))
        (:`NewEnumerator8`
          ;[1 1 1] Leash
          (`/Game/Mods/SexilesMod/ActorComponents/ac_SXM_Leash.MakeRopeConnection` (`Actor.GetComponentByClass` (`self.GetOwner`) "/Game/Mods/SexilesMod/ActorComponents/ac_SXM_Leash.ac_SXM_Leash_C") (`self.TargetNPC`)))
        (:`NewEnumerator13`
          ;[1 1 1] Seduce - Passive
          (bind _assxm_bp_pc (cast `/Game/Mods/SexilesMod/Character/SXM_BP_PC` (`self.GetOwner`) :!label _label_2))
          (`/Engine/EditorBlueprintResources/StandardMacros.IsValid` (`self.TargetNPC`)
            (:`Is Valid`
              (`/Game/Mods/SexilesMod/Character/SXM_BP_PC.SXM_NPCInteraction handle` _assxm_bp_pc (`|EnumEquality` CategoryID "NewEnumerator13") (`self.MenuSelectedAnimationIndex`) (`Actor.GetComponentByClass` (`self.TargetNPC`) "/Game/Mods/SexilesMod/Character/SXM_Component.SXM_Component_C")))))
        (:`NewEnumerator3`
          (goto _label_2))))))

(fn `GetSXMTableValues`
  (params (ActorCount :type Integer) (RowName :type Name))
  (returns (ReturnValue :type Boolean) (DisplayName :type Text) (EmoteCategory :type Text) (Icon :type "Texture2D Object Reference"))
  (if (`|EnumEquality` (`UserSettingsLibrary.GetNudityLevel`) "Full")
    (bind _returnvalue (`|GetDataTableRow` "/Game/Mods/SexilesMod/Character/SXM_AnimsData.SXM_AnimsData" RowName)
      (:`then`
        _)
      (:`RowNotFound`
        _))
    (bind (_animdescription _displayname _emotecategory _iconpassive _iconactive _animstagecount _isfirstactorpenetrator _isdisabled _actorcount) (break `/Game/Mods/SexilesMod/Character/SXM_AnimStruct` _returnvalue))
    (return (and (not _isdisabled) (== _actorcount ActorCount)) (`KismetTextLibrary.Conv_StringToText` _displayname) (`KismetTextLibrary.Conv_StringToText` _emotecategory) _iconpassive)
    (else
      (bind _returnvalue_2 (`|GetDataTableRow` "/Game/Mods/SexilesMod/Character/SXM_AnimsData_SFW.SXM_AnimsData_SFW" RowName)
        (:`then`
          _)
        (:`RowNotFound`
          _))
      (bind (_animdescription_2 _displayname_2 _emotecategory_2 _iconpassive_2 _iconactive_2 _animstagecount_2 _isfirstactorpenetrator_2 _isdisabled_2 _actorcount_2) (break `/Game/Mods/SexilesMod/Character/SXM_AnimStruct` _returnvalue_2))
      (return (and (not _isdisabled_2) (== _actorcount_2 ActorCount)) (`KismetTextLibrary.Conv_StringToText` _displayname_2) (`KismetTextLibrary.Conv_StringToText` _emotecategory_2) _iconpassive_2))))

(fn `OnRep_NewVar_0`)