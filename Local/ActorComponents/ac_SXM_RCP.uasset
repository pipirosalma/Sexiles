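; Player character component that tracks Tied Up, Drugged and Drunken status flags and grants sleep recovery.
; Buff-added signals set Tied Up, and Drunken from drunk stage three; nothing here sets Drugged.
; Tick clears either flag when its buff check returns true, as written, and relays changes through SetVariables_SRV to SetVariables_C.
; Substate events add a healing recovery buff during the SleepOnGround emote and remove it on exit.
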(event `self.ReceiveBeginPlay`
  (bind _asbase_player_char (`self.GetBasePlayerChar`))
  (bind _00_bp_ac_buffsystem (`/Game/Characters/BaseBPCombat.00_BP_AC_BuffSystem` _asbase_player_char))
  (set `self.BPACBuffSystem` _00_bp_ac_buffsystem)
  (add `/Game/Systems/Buffs/00_BP_AC_BuffSystem.SignalBuffAdded` _00_bp_ac_buffsystem (delegate `RegisterBuff`))
  (add `/Game/Characters/BaseBPChar.OnCharacterSubstateChanged` _asbase_player_char (delegate `EmoteCheck`)))

(event `RegisterBuff`
  (params (buff :type "/Game/Systems/Buffs/01_BP_AC_Buff_Master Object Reference"))
  (`|ExecutionSequence`
    (:`then_0`
      ;[1 1 1] Drunken Flag
      (cast `/Game/Mods/SexilesMod/System/BP_Buff_Tied_Up` buff)
      (set `self.TiedUp` true)
      (set `self.UpdateFlag` true))
    (:`then_1`
      (bind _asbp_ac_buff_drunkenness (cast `/Game/Systems/Buffs/Alcohol/BP_AC_Buff_Drunkenness` buff))
      (set `self.Drunken` (>= (`/Game/Systems/Buffs/Alcohol/BP_AC_Buff_Drunkenness.DrunkStage` _asbp_ac_buff_drunkenness) 3))
      (set `self.UpdateFlag` true))))

(event `SetVariables_SRV`
  (params (TiedUp :type Boolean) (Drugged :type Boolean) (Drunken :type Boolean))
  ;[1 1 1] Drunken Flag
  (`self.SetVariables_C` TiedUp Drugged Drunken))

(event `SetVariables_C`
  (params (TiedUp :type Boolean) (Drugged :type Boolean) (Drunken :type Boolean))
  ;[1 1 1] Drunken Flag
  (set `self.TiedUp` TiedUp)
  (set `self.Drugged` Drugged)
  (set `self.Drunken` Drunken))

(event `EmoteCheck`
  (params (Substate :type "/Game/Characters/CharacterSubState Enum") (Entered :type Boolean))
  (bind _asbase_player_char (`self.GetBasePlayerChar`))
  ;[1 1 1] Sleep Recovery
  (`/Game/Systems/BP_MacroGlobal.And+Branch` (`|EnumEquality` Substate "NewEnumerator5") Entered
    (:`True`
      (bind _newparam (`/Game/Characters/BaseBPCombat.GetCurrentEmote` (`self.GetBasePlayerChar`)))
      (if (`|EnumEquality` _newparam "SleepOnGround")
        (`/Game/Systems/Buffs/00_BP_AC_BuffSystem.AddBuff` (`/Game/Characters/BaseBPCombat.00_BP_AC_BuffSystem` _asbase_player_char) "/Game/Mods/SexilesMod/System/BP_AC_Buff_HealingRecovery.BP_AC_Buff_HealingRecovery_C" null 1 null)
        (add `/Game/Characters/BaseBPChar.OnCharacterSubstateChanged` _asbase_player_char (delegate `RemoveRecovery`))))))

(event `RemoveRecovery`
  (params (Substate :type "/Game/Characters/CharacterSubState Enum") (Entered :type Boolean))
  (bind _asbase_player_char (`self.GetBasePlayerChar`))
  ;[1 1 1] Sleep Recovery
  (`/Game/Systems/BP_MacroGlobal.And+Branch` (`|EnumEquality` Substate "NewEnumerator5") (not Entered)
    (:`True`
      (`/Game/Systems/Buffs/00_BP_AC_BuffSystem.RemoveBuff` (`/Game/Characters/BaseBPCombat.00_BP_AC_BuffSystem` _asbase_player_char) "/Game/Mods/SexilesMod/System/BP_AC_Buff_HealingRecovery.BP_AC_Buff_HealingRecovery_C")
      (remove `/Game/Characters/BaseBPChar.OnCharacterSubstateChanged` _asbase_player_char (delegate `RemoveRecovery`)))))

(event `self.ReceiveTick`
  (params (DeltaSeconds :type "Float (single-precision)"))
  ;[1 1 1] BuffCheck /w flags
  (`|ExecutionSequence`
    (:`then_0`
      (if (`self.TiedUp`)
        (if (`/Game/Systems/Buffs/00_BP_AC_BuffSystem.CheckIfBuffExists` (`self.BPACBuffSystem`) "/Game/Mods/SexilesMod/System/BP_Buff_Tied_Up.BP_Buff_Tied_Up_C")
          (set `self.TiedUp` false)
          (set `self.UpdateFlag` true))))
    (:`then_1`
      (if (`self.Drunken`)
        (if (`/Game/Systems/Buffs/00_BP_AC_BuffSystem.CheckIfBuffExists` (`self.BPACBuffSystem`) "/Game/Systems/Buffs/Alcohol/BP_AC_Buff_Drunkenness.BP_AC_Buff_Drunkenness_C")
          (set `self.Drunken` false)
          (set `self.UpdateFlag` true))))
    (:`then_3`
      (if (`self.UpdateFlag`)
        (`self.SetVariables_SRV` (`self.TiedUp`) (`self.Drugged`) (`self.Drunken`))
        (set `self.UpdateFlag` false)))))

(fn `GetBasePlayerChar`
  (returns (`AsBase Player Char` :type "/Game/Characters/BasePlayerChar Object Reference"))
  (bind _asbase_player_char (cast `/Game/Characters/BasePlayerChar` (`self.GetOwner`))
    (:`then`
      _)
    (:`CastFailed`
      _))
  (return _asbase_player_char))

(fn `OnRep_TiedUp`)

(fn `OnRep_UpdateFlag`)