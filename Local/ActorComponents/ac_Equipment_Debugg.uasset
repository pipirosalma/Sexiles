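; Actor component on the player character that, judging by its name, is a debug helper for equipment changes.
; On BeginPlay it casts the owner to BasePlayerChar and binds to the Equipment inventory's item added and removed signals.
; Both signals share one path: if the character's SXMComponent is activated, the mesh's anim instance class is set to SXM_AB again.
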(event `self.ReceiveBeginPlay`
  (bind _asbase_player_char (cast `/Game/Characters/BasePlayerChar` (`self.GetOwner`)))
  (bind _returnvalue (`ItemInventory.GetInventoryByType` _asbase_player_char "Equipment"))
  (add `ItemInventory.SignalItemAdded` _returnvalue (delegate `SignalItemAdded_Event_0`))
  (add `ItemInventory.SignalItemRemoved` _returnvalue (delegate `SignalItemRemoved_Event_0`)))

(event `SignalItemAdded_Event_0`
  (params (index :type Integer) (item :type "GameItem Object Reference") (srcInventory :type "ItemInventory Object Reference") (srcIndex :type Integer))
  (if (`/Game/Mods/SexilesMod/Character/SXM_Component.IsActivated` (`/Game/Mods/SexilesMod/Character/SXM_BP_PC.SXM_Component` (stale `self.ReceiveBeginPlay` _asbase_player_char))) :!label _label
    (`SkeletalMeshComponent.SetAnimInstanceClass` (`Character.Mesh` (stale `self.ReceiveBeginPlay` _asbase_player_char)) "/Game/Mods/SexilesMod/Character/SXM_AB.SXM_AB_C")))

(event `SignalItemRemoved_Event_0`
  (params (index :type Integer) (item :type "GameItem Object Reference") (dstInventory :type "ItemInventory Object Reference") (dstIndex :type Integer))
  (goto _label))