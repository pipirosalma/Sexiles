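; Actor component on a weapon that assigns the Knockout debuff as the wielder's main-hand buff class for truncheons and the "Lovetap" club.
; On BeginPlay it casts its owner to the one-handed truncheon, or to a one-handed club whose item name matches, then reaches the owning player character.
; Dedicated servers apply this only with PVP enabled, while all other instances always apply it.
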(event `self.ReceiveBeginPlay`
  (bind _returnvalue (`self.GetOwner`))
  (if (`KismetSystemLibrary.IsDedicatedServer`)
    (if (`ServerSettings.PVPEnabled` (`|GetServerSettings`))
      (bind _asbp_truncheon_1h (cast `/Game/Items/Weapons/Club/BP_truncheon_1h` _returnvalue :!label _label)
        (:`then`
          (bind _asbase_player_char (cast `/Game/Characters/BasePlayerChar` (`Actor.GetOwner` _asbp_truncheon_1h)))
          (set `/Game/Items/BPGameItemWeapon.BuffClass` "/Game/Mods/SexilesMod/System/BP_AC_Debuff_Knockout.BP_AC_Debuff_Knockout_C" (`/Game/Characters/BaseBPCombat.GetMainhandWeapon` _asbase_player_char)))
        (:`CastFailed`
          (bind _asbp_club_1h (cast `/Game/Items/Weapons/Club/BP_club_1h` _returnvalue))
          (if (`KismetTextLibrary.EqualEqual_TextText` (`GameItem.Name` (`/Game/Items/Weapons/BaseHitActor.GetOwnerWeaponItem` _asbp_club_1h)) "Lovetap")
            (bind _asbase_player_char_2 (cast `/Game/Characters/BasePlayerChar` (`Actor.GetOwner` _asbp_club_1h)))
            (set `/Game/Items/BPGameItemWeapon.BuffClass` "/Game/Mods/SexilesMod/System/BP_AC_Debuff_Knockout.BP_AC_Debuff_Knockout_C" (`/Game/Characters/BaseBPCombat.GetMainhandWeapon` _asbase_player_char_2))))))
    (else
      (goto _label))))