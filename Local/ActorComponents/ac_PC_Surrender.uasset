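; Player surrender component that hands a selected humanoid NPC to the SXM interaction system and can refresh an offender's outfit.
; Surrender reacts to a substate entry during the Flirt1 emote, setting the role by player gender, but its binding is never run.
; Undress chains through SRV and C events to force-reapply the offender's existing layout and update meshes.
; A helper picks random animations from bound-variation table rows.
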(event `Undress`
  (params (Offender :type "/Game/Characters/NPCs/Humanoid/BaseHumanoidNPC Object Reference"))
  (`self.UndressSRV` Offender))

(event `UndressSRV`
  (params (Offender :type "/Game/Characters/NPCs/Humanoid/BaseHumanoidNPC Object Reference"))
  (`self.UndressC` Offender))

(event `UndressC`
  (params (Offender :type "/Game/Characters/NPCs/Humanoid/BaseHumanoidNPC Object Reference"))
  (`self.ExeUndress` Offender))

(event `self.ReceiveBeginPlay`)

(event `Surrender`
  (params (Substate :type "/Game/Characters/CharacterSubState Enum") (Entered :type Boolean))
  (bind _owningbaseplayer (`self.OwningBasePlayer`))
  (`/Game/Systems/BP_MacroGlobal.And+Branch` (`|EnumEquality` Substate "NewEnumerator5") Entered
    (:`True`
      (bind _newparam (`/Game/Characters/BaseBPCombat.GetCurrentEmote` (`self.OwningBasePlayer`)))
      (if (`|EnumEquality` _newparam "Flirt1")
        (bind _asfun_combat_player_controller (cast `/Game/Systems/FunCombat_PlayerController` (`/Game/Characters/FuncomFunctionLibrary.GetControllerFromActor` (`self.GetOwner`))))
        (bind _returnvalue (`/Game/Systems/FunCombat_PlayerController.GetInteractionManager` _asfun_combat_player_controller))
        (if (`/Game/Systems/InteractionManager.HasSelectedObject` _returnvalue)
          (bind _asbase_humanoid_npc (cast `/Game/Characters/NPCs/Humanoid/BaseHumanoidNPC` (`KismetSystemLibrary.Conv_InterfaceToObject` (`/Game/Systems/InteractionManager.SelectedObject` _returnvalue))))
          (bind _returnvalue_2 (`Actor.GetComponentByClass` _asbase_humanoid_npc "/Game/Mods/SexilesMod/Character/SXM_Component.SXM_Component_C"))
          (`/Engine/EditorBlueprintResources/StandardMacros.IsValid` _returnvalue_2
            (:`Is Valid`
              (set `/Game/Mods/SexilesMod/Character/SXM_Component.AutoDress` true _returnvalue_2)
              (`/Game/Mods/SexilesMod/Character/SXM_BP_PC.SXM_NPCInteraction handle` _owningbaseplayer (not (break `CharacterBoolParameters` (`.BoolParams` (break `CharacterLayout` (`/Game/Characters/BasePlayerChar.CharacterLayout` _owningbaseplayer))))) 4 _returnvalue_2))))))))

(fn `ExeUndress`
  (params (Offender :type "/Game/Characters/NPCs/Humanoid/BaseHumanoidNPC Object Reference"))
  (bind _returnvalue (`Actor.GetComponentByClass` Offender "/Game/Characters/BP_CharacterCustomizationComponent.BP_CharacterCustomizationComponent_C"))
  (bind (_meshlayout _texturelayout _tintlayout _boolparams _intparams _scalarparams _enumparams _armourdyeparams) (break `CharacterLayout` (`CharacterCustomizationComponent.Layout` _returnvalue)))
  (bind (_helmet _hair _facialhair _head _forearms _hands _upperbody _lowerbody _legs _feet) (break `CharacterMeshLayout` _meshlayout))
  (`CharacterCustomizationComponent.SetCharacterLayout` _returnvalue (make `CharacterLayout` (make `CharacterMeshLayout` _helmet _hair _facialhair _head _forearms _hands _upperbody 0 _legs _feet) _texturelayout _tintlayout _boolparams _intparams _scalarparams _enumparams _armourdyeparams) true true)
  (`/Game/Characters/NPCs/Humanoid/BaseHumanoidNPC.UpdateMeshes` Offender))