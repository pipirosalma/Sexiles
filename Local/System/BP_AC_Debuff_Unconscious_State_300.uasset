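; Debuff component that keeps a player character unconscious for as long as the buff is active.
; On start it caches the owner; the start visual-effect event triggers unconsciousness and plays a bound-kneel montage.
; It binds to character state changes to reapply unconsciousness whenever the state switches to anything else.
; The clear event lifts unconsciousness, unbinds that listener and stops the montage.
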(event `self.StartBuff`
  (params (BuffPotency :type Integer) (DamageCauser :type "Actor Object Reference") (OwningCharacter :type "ConanCharacter Object Reference") (Instigator :type "Controller Object Reference"))
  (`parent.StartBuff` BuffPotency DamageCauser OwningCharacter Instigator)
  (bind _asbase_player_char (cast `/Game/Characters/BasePlayerChar` (`self.OwningCharacter`)))
  (set `self.OwningBasePC` _asbase_player_char))

(event `self.MulticastVisualEffectToApplyOnBuffStart`
  (bind _asbase_player_char (cast `/Game/Characters/BasePlayerChar` (`self.OwningCharacter`)))
  (`/Game/Mods/SexilesMod/Character/SXM_BP_PC.HandleUnconsciousEvent` _asbase_player_char true)
  (add `ConanCharacter.OnCharacterStateChanged` _asbase_player_char (delegate `Knockrepeat`))
  (`Character.PlayAnimMontage` (`self.OwningBasePC`) "/Game/Mods/SexilesMod/Character/Anims/Poses/SXM_Bound_Kneel_v2.SXM_Bound_Kneel_v2" 1.0 "None"))

(event `Knockrepeat`
  (params (OldState :type "ECharacterState Enum") (NewState :type "ECharacterState Enum"))
  (if (`|EnumInequality` NewState "Unconscious")
    (`/Game/Mods/SexilesMod/Character/SXM_BP_PC.HandleUnconsciousEvent` (stale `self.MulticastVisualEffectToApplyOnBuffStart` _asbase_player_char) true)))

(event `self.MulticastVisualEffectToApplyOnBuffCleared`
  (bind _asbase_player_char (cast `/Game/Characters/BasePlayerChar` (`self.OwningCharacter`)))
  (`/Game/Mods/SexilesMod/Character/SXM_BP_PC.HandleUnconsciousEvent` _asbase_player_char false)
  (remove `ConanCharacter.OnCharacterStateChanged` _asbase_player_char (delegate `Knockrepeat`))
  (`Character.StopAnimMontage` (`self.OwningBasePC`) "/Game/Mods/SexilesMod/Character/Anims/Poses/SXM_Bound_Kneel_v2.SXM_Bound_Kneel_v2"))