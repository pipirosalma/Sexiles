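; Buff Blueprint for the "Deadly Kiss" effect that temporarily changes the owning player character's lip appearance.
; On buff start, it saves the character layout's lip texture and lip makeup tint, then rebuilds the layout with fixed replacements for both.
; On clear, it rebuilds the current layout with the saved values, leaving all other fields as they are.
; Both events require a BasePlayerChar owner and call the parent buff logic afterward.
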(event `/Game/Systems/Buffs/01_BP_AC_Buff_Master.GameplayEffectToApplyOnBuffStart`
  (bind _asbase_player_char (cast `/Game/Characters/BasePlayerChar` (`self.GetOwner`)))
  (bind _character_layout (`/Game/Characters/BasePlayerChar.GetCharacterLayout` _asbase_player_char))
  (bind (_meshlayout _texturelayout _tintlayout _boolparams _intparams _scalarparams _enumparams _armourdyeparams) (break `CharacterLayout` _character_layout))
  (bind (_eyebrowtexture _eyetexture _liptexture _warpaintfacetexture _warpaintbodytexture _warpainthandstexture _hairlinetexture _facialhairlinetexture) (break `CharacterTextureLayout` _texturelayout))
  (set `self.liptexture` _liptexture)
  (bind (_skin _hair _facialhair _eyes _eyebrows _eyemakeup _lipmakeup _warpaint) (break `CharacterTintLayout` _tintlayout))
  (set `self.colorsaveint` _lipmakeup)
  (`/Game/Characters/BasePlayerChar.SetCharacterLayout` _asbase_player_char (make `CharacterLayout` _meshlayout (make `CharacterTextureLayout` _eyebrowtexture _eyetexture 2 _warpaintfacetexture _warpaintbodytexture _warpainthandstexture _hairlinetexture _facialhairlinetexture) (make `CharacterTintLayout` _skin _hair _facialhair _eyes _eyebrows _eyemakeup 8 _warpaint) _boolparams _intparams _scalarparams _enumparams _armourdyeparams))
  (`parent.GameplayEffectToApplyOnBuffStart`))

(event `/Game/Systems/Buffs/01_BP_AC_Buff_Master.GameplayEffectToApplyOnBuffCleared`
  (bind _asbase_player_char (cast `/Game/Characters/BasePlayerChar` (`self.GetOwner`)))
  (bind _character_layout (`/Game/Characters/BasePlayerChar.GetCharacterLayout` _asbase_player_char))
  (bind (_meshlayout _texturelayout _tintlayout _boolparams _intparams _scalarparams _enumparams _armourdyeparams) (break `CharacterLayout` _character_layout))
  (bind (_eyebrowtexture _eyetexture _liptexture _warpaintfacetexture _warpaintbodytexture _warpainthandstexture _hairlinetexture _facialhairlinetexture) (break `CharacterTextureLayout` _texturelayout))
  (bind (_skin _hair _facialhair _eyes _eyebrows _eyemakeup _lipmakeup _warpaint) (break `CharacterTintLayout` _tintlayout))
  (`/Game/Characters/BasePlayerChar.SetCharacterLayout` _asbase_player_char (make `CharacterLayout` _meshlayout (make `CharacterTextureLayout` _eyebrowtexture _eyetexture (`self.liptexture`) _warpaintfacetexture _warpaintbodytexture _warpainthandstexture _hairlinetexture _facialhairlinetexture) (make `CharacterTintLayout` _skin _hair _facialhair _eyes _eyebrows _eyemakeup (`self.colorsaveint`) _warpaint) _boolparams _intparams _scalarparams _enumparams _armourdyeparams))
  (`parent.GameplayEffectToApplyOnBuffCleared`))