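; Debuff component that keeps a player character unconscious for as long as the buff is active.
; On buff start, its multicast visual-effect event triggers the unconscious event on BasePlayerChar and binds to character state changes.
; Any change to a state other than Unconscious re-triggers the knockout.
; Clearing the buff turns the unconscious event off and unbinds the listener.
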(event `self.StartBuff`
  (params (BuffPotency :type Integer) (DamageCauser :type "Actor Object Reference") (OwningCharacter :type "ConanCharacter Object Reference") (Instigator :type "Controller Object Reference"))
  (`parent.StartBuff` BuffPotency DamageCauser OwningCharacter Instigator))

(event `self.MulticastVisualEffectToApplyOnBuffStart`
  (bind _asbase_player_char (cast `/Game/Characters/BasePlayerChar` (`self.OwningCharacter`)))
  (`/Game/Mods/SexilesMod/Character/SXM_BP_PC.HandleUnconsciousEvent` _asbase_player_char true)
  (add `ConanCharacter.OnCharacterStateChanged` _asbase_player_char (delegate `Knockrepeat`)))

(event `Knockrepeat`
  (params (OldState :type "ECharacterState Enum") (NewState :type "ECharacterState Enum"))
  (if (`|EnumInequality` NewState "Unconscious")
    (`/Game/Mods/SexilesMod/Character/SXM_BP_PC.HandleUnconsciousEvent` (stale `self.MulticastVisualEffectToApplyOnBuffStart` _asbase_player_char) true)))

(event `self.MulticastVisualEffectToApplyOnBuffCleared`
  (bind _asbase_player_char (cast `/Game/Characters/BasePlayerChar` (`self.OwningCharacter`)))
  (`/Game/Mods/SexilesMod/Character/SXM_BP_PC.HandleUnconsciousEvent` _asbase_player_char false)
  (remove `ConanCharacter.OnCharacterStateChanged` _asbase_player_char (delegate `Knockrepeat`)))