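; Temporary fluid-stain decal actor that animates over a timeline and then destroys itself.
; On BeginPlay it creates a dynamic material instance and picks a random stain channel for variation.
; Bloodstain_timeline updates the material's opacity and life parameters until it finishes.
; AttachDecalToActor attaches the decal to a supplied component socket, keeping its relative transform.
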(event `AttachDecalToActor`
  (params (actor :type "SceneComponent Object Reference") (socketname :type Name))
  (`SceneComponent.K2_AttachToComponent` (`self.Decal`) actor socketname "KeepRelative" "KeepRelative" "KeepRelative" true))

(event `self.ReceiveBeginPlay`
  (bind _returnvalue (`DecalComponent.CreateDynamicMaterialInstance` (`self.Decal`)))
  (`MaterialInstanceDynamic.SetScalarParameterValue` _returnvalue "stain_channel" (`KismetMathLibrary.Conv_IntToDouble` (`KismetMathLibrary.RandomIntegerInRange` 0 3)))
  (bind (_direction _life) (`Timeline|bloodstain_timeline` :!via `PlayFromStart`)
    (:`Update`
      (`MaterialInstanceDynamic.SetScalarParameterValue` _returnvalue "stain_opacity" (`self.stain_opacity`))
      (`MaterialInstanceDynamic.SetScalarParameterValue` _returnvalue "stain_life" _life))
    (:`Finished`
      (`self.K2_DestroyActor`))))

(fn `UserConstructionScript`)