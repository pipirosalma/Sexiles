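; Stacking buff for an adult "cum covered" status, shown on the owning character through the warpaint layer.
; On start and after each stack adjustment, it edits the owner's layout message, setting face and body warpaint textures and tint to stack size plus a fixed ID offset.
; Hand warpaint is always zeroed.
; Clearing zeroes all these slots rather than restoring the prior warpaint, as the saved layout is never read.
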(event `self.GameplayEffectToApplyOnBuffStart`
  (bind _returnvalue (+ (`self.StackSize`) 1920))
  (bind _character_layout (message `/Game/Characters/I_HasCharacterLayoutInterface.GetCharacterLayout` (`self.GetOwner`)))
  (set `self.savedlayout` _character_layout)
  (bind _output_get (set `self.Layout` _character_layout))
  (`CharacterFunctionLibrary.SetCharacterTextureSlot` (`.TextureLayout` (break `CharacterLayout` _output_get)) "WarpaintFace" _returnvalue)
  (`CharacterFunctionLibrary.SetCharacterTextureSlot` (`.TextureLayout` (break `CharacterLayout` _output_get)) "WarpaintBody" _returnvalue)
  (`CharacterFunctionLibrary.SetCharacterTintSlot` (`.TintLayout` (break `CharacterLayout` _output_get)) "Warpaint" _returnvalue)
  (`CharacterFunctionLibrary.SetCharacterTextureSlot` (`.TextureLayout` (break `CharacterLayout` _output_get)) "WarpaintHands")
  (message `/Game/Characters/I_HasCharacterLayoutInterface.SetCharacterLayout` (`self.GetOwner`) (`self.Layout`)))

(event `self.GameplayEffectToApplyOnBuffCleared`
  (bind _character_layout (message `/Game/Characters/I_HasCharacterLayoutInterface.GetCharacterLayout` (`self.GetOwner`)))
  (set `self.savedlayout` _character_layout)
  (bind _output_get (set `self.Layout` _character_layout))
  (`CharacterFunctionLibrary.SetCharacterTextureSlot` (`.TextureLayout` (break `CharacterLayout` _output_get)) "WarpaintFace")
  (`CharacterFunctionLibrary.SetCharacterTextureSlot` (`.TextureLayout` (break `CharacterLayout` _output_get)) "WarpaintBody")
  (`CharacterFunctionLibrary.SetCharacterTintSlot` (`.TintLayout` (break `CharacterLayout` _output_get)) "Warpaint")
  (`CharacterFunctionLibrary.SetCharacterTextureSlot` (`.TextureLayout` (break `CharacterLayout` _output_get)) "WarpaintHands")
  (message `/Game/Characters/I_HasCharacterLayoutInterface.SetCharacterLayout` (`self.GetOwner`) (`self.Layout`)))

(event `self.AdjustStackSize`
  (params (StackAdjustment :type Integer))
  (bind _returnvalue (+ (`self.StackSize`) 1920))
  (`parent.AdjustStackSize` StackAdjustment)
  (bind _character_layout (message `/Game/Characters/I_HasCharacterLayoutInterface.GetCharacterLayout` (`self.GetOwner`)))
  (set `self.savedlayout` _character_layout)
  (bind _output_get (set `self.Layout` _character_layout))
  (`CharacterFunctionLibrary.SetCharacterTextureSlot` (`.TextureLayout` (break `CharacterLayout` _output_get)) "WarpaintFace" _returnvalue)
  (`CharacterFunctionLibrary.SetCharacterTextureSlot` (`.TextureLayout` (break `CharacterLayout` _output_get)) "WarpaintBody" _returnvalue)
  (`CharacterFunctionLibrary.SetCharacterTintSlot` (`.TintLayout` (break `CharacterLayout` _output_get)) "Warpaint" _returnvalue)
  (`CharacterFunctionLibrary.SetCharacterTextureSlot` (`.TextureLayout` (break `CharacterLayout` _output_get)) "WarpaintHands")
  (message `/Game/Characters/I_HasCharacterLayoutInterface.SetCharacterLayout` (`self.GetOwner`) (`self.Layout`)))