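; Rope weapon Blueprint that switches the player's rope animation state and rope visual on equip and unequip.
; Equip sets RopeEquiped on the character's Ac_AditionalAnimations component, runs the parent logic, then connects the rope on the BP_rope_1h_new visual actor.
; Unequip clears the flag and destroys the rope before running the parent logic.
; Also holds an owner-to-BasePlayerChar lookup and a capsule-location trace-start macro, neither used by these events.
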(event `self.OnEquip`
  (params (owner :type "Character Object Reference"))
  (bind _asbase_player_char (cast `/Game/Characters/BasePlayerChar` owner)
    (:`then`
      (bind _returnvalue (`Actor.K2_GetComponentsByClass` _asbase_player_char "/Game/Mods/SexilesMod/ac_AditionalAnimations.ac_AditionalAnimations_C"))
      (if (> (`KismetArrayLibrary.Array_Length` _returnvalue) 0)
        (set `/Game/Mods/SexilesMod/ac_AditionalAnimations.RopeEquiped` true (`KismetArrayLibrary.Array_Get` _returnvalue))))
    (:`CastFailed`
      _))
  (`parent.OnEquip` owner)
  (bind _asbp_rope_1h_new (cast `/Game/Mods/SexilesMod/Weapons/BP_rope_1h_new` (`self.GetVisualWeapon`)))
  (`/Game/Mods/SexilesMod/Weapons/BP_rope_1h_new.MakeRopeConnection` _asbp_rope_1h_new))

(event `self.OnUnEquip`
  (params (owner :type "Character Object Reference"))
  (bind _asbase_player_char (cast `/Game/Characters/BasePlayerChar` owner)
    (:`then`
      (bind _returnvalue (`Actor.K2_GetComponentsByClass` _asbase_player_char "/Game/Mods/SexilesMod/ac_AditionalAnimations.ac_AditionalAnimations_C"))
      (if (> (`KismetArrayLibrary.Array_Length` _returnvalue) 0)
        (set `/Game/Mods/SexilesMod/ac_AditionalAnimations.RopeEquiped` false (`KismetArrayLibrary.Array_Get` _returnvalue))))
    (:`CastFailed`
      _))
  (bind _asbp_rope_1h_new (cast `/Game/Mods/SexilesMod/Weapons/BP_rope_1h_new` (`self.GetVisualWeapon`))
    (:`then`
      (`/Game/Mods/SexilesMod/Weapons/BP_rope_1h_new.destroyrope` _asbp_rope_1h_new))
    (:`CastFailed`
      _))
  (`parent.OnUnEquip` owner))

(fn `GetBasePlayerChar`
  (returns (BasePlayerChar :type "/Game/Characters/BasePlayerChar Object Reference"))
  (bind _returnvalue (`self.GetOwner`))
  (bind _asfun_combat_player_controller (cast `/Game/Systems/FunCombat_PlayerController` _returnvalue)
    (:`then`
      (cast `/Game/Characters/BasePlayerChar` (`Controller.K2_GetPawn` _asfun_combat_player_controller)
        (:`then`
          _)
        (:`CastFailed`
          _)))
    (:`CastFailed`
      (bind _asbase_player_char (cast `/Game/Characters/BasePlayerChar` _returnvalue)
        (:`then`
          _)
        (:`CastFailed`
          _))))
  (return _asbase_player_char))