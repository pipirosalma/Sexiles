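; BP_AC_Buff_Shackled is a buff that snares the owning character by adjusting its movement speed multiplier with SnareValue.
; It caches the owner's combat interface on init and client start, applies the snare on buff start with DoesNotExpire set, and removes it on clear.
; Client start and clear events reuse the same apply and remove logic only off the server, preventing a double application on a listen host.
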(event `self.InitBuff`
  (params (DamageCauser :type "Actor Object Reference") (OwningCharacter :type "ConanCharacter Object Reference") (Instigator :type "Controller Object Reference"))
  (`parent.InitBuff` null OwningCharacter Instigator)
  (bind _asis_base_bpcombat_interface (cast `/Game/Systems/Interfaces/IsBaseBPCombatInterface` (`self.OwningCharacter`)))
  (set `self.ConbatInterface` _asis_base_bpcombat_interface))

(event `EffectToApplyOnBuffTick`)

(event `self.GameplayEffectToApplyOnBuffStart`
  (`parent.GameplayEffectToApplyOnBuffStart`)
  (bind _output_get (set `self.DoesNotExpire` true :!label _label))
  (`/Game/Systems/Interfaces/IsBaseBPCombatInterface.AdjustMovementSpeedMultiplier` (`self.ConbatInterface`) _output_get (`self.SnareValue`)))

(event `self.ClientStartBuff`
  (params (OwningCharacter :type "ConanCharacter Object Reference") (Duration :type "Float (single-precision)"))
  (`parent.ClientStartBuff` OwningCharacter Duration)
  (bind _asis_base_bpcombat_interface (cast `/Game/Systems/Interfaces/IsBaseBPCombatInterface` (`self.OwningCharacter`)))
  (set `self.ConbatInterface` _asis_base_bpcombat_interface)
  ;[1 1 1] If we didn’t do this; then it would apply the effect twice
  (if (not (`KismetSystemLibrary.IsServer`))
    (goto _label)))

(event `self.GameplayEffectToApplyOnBuffCleared`
  (`parent.GameplayEffectToApplyOnBuffCleared`)
  (`/Game/Systems/Interfaces/IsBaseBPCombatInterface.AdjustMovementSpeedMultiplier` (`self.ConbatInterface`) false (`self.SnareValue`) :!label _label_2))

(event `self.ClientClearBuff`
  (params (OwningCharacter :type "ConanCharacter Object Reference"))
  (`parent.ClientClearBuff` OwningCharacter)
  ;[1 1 1] If we didn’t do this; then it would apply the effect twice
  (if (not (`KismetSystemLibrary.IsServer`))
    (goto _label_2)))