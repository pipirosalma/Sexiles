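; Handcuff equipment item that restrains its wearer with a hands-bound-behind-back pose.
; On equip it plays the bound montage on the combat character owner and adds the handcuffed buff through the buff system component; unequip stops the montage and removes that buff.
; Helper graphs for sequence-based montage selection and additional-animation component lookup are present but not called by the equip events, and the AnimSequence OnRep is empty.
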(event `self.OnEquip`
  (params (owner :type "Character Object Reference"))
  (`parent.OnEquip` owner)
  (bind _asbase_bpcombat (cast `/Game/Characters/BaseBPCombat` owner))
  (`Character.PlayAnimMontage` _asbase_bpcombat "/Game/Mods/SexilesMod/Animation_Temp/AM_Behind_Back_Bound.AM_Behind_Back_Bound" 1.0 "None")
  (`/Game/Systems/Buffs/00_BP_AC_BuffSystem.AddBuff` (`/Game/Characters/BaseBPCombat.00_BP_AC_BuffSystem` _asbase_bpcombat) "/Game/Mods/SexilesMod/Armors/Chains/BP_AC_Buff_handcuffed.BP_AC_Buff_handcuffed_C" null 0 null))

(event `self.OnUnEquip`
  (params (owner :type "Character Object Reference"))
  (`parent.OnUnEquip` owner)
  (`Character.StopAnimMontage` owner "/Game/Mods/SexilesMod/Animation_Temp/AM_Behind_Back_Bound.AM_Behind_Back_Bound")
  (bind _asbase_bpcombat (cast `/Game/Characters/BaseBPCombat` owner))
  (`/Game/Systems/Buffs/00_BP_AC_BuffSystem.RemoveBuff` (`/Game/Characters/BaseBPCombat.00_BP_AC_BuffSystem` _asbase_bpcombat) "/Game/Mods/SexilesMod/Armors/Chains/BP_AC_Buff_handcuffed.BP_AC_Buff_handcuffed_C"))

(fn `OnRep_AnimSequence`)