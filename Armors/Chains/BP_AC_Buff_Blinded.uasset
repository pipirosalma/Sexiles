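; Blinded buff Blueprint that makes a player character play a sitting prayer montage and adjusts its movement speed while active.
; Start sets DoesNotExpire and applies a speed multiplier adjustment of 1.0; clearing stops the montage and removes the adjustment using SnareValue.
; Client start and clear events reuse the effect logic only off-server, avoiding double application.
; Tick does nothing, and the full-screen effect call is disconnected.
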(event `self.InitBuff`
  (params (DamageCauser :type "Actor Object Reference") (OwningCharacter :type "ConanCharacter Object Reference") (Instigator :type "Controller Object Reference"))
  (`parent.InitBuff` null OwningCharacter Instigator)
  (bind _asis_base_bpcombat_interface (cast `/Game/Systems/Interfaces/IsBaseBPCombatInterface` (`self.OwningCharacter`)))
  (set `self.ConbatInterface` _asis_base_bpcombat_interface))

(event `EffectToApplyOnBuffTick`)

(event `self.GameplayEffectToApplyOnBuffStart`
  (`parent.GameplayEffectToApplyOnBuffStart`)
  (bind _output_get (set `self.DoesNotExpire` true :!label _label))
  (bind _asbase_player_char (cast `/Game/Characters/BasePlayerChar` (`self.OwningCharacter`)))
  (`Character.PlayAnimMontage` _asbase_player_char "/Game/Characters/humans/animations/emotes/AM_emote_pray_sitting.AM_emote_pray_sitting" 1.0 "None")
  (`/Game/Systems/Interfaces/IsBaseBPCombatInterface.AdjustMovementSpeedMultiplier` (`self.ConbatInterface`) _output_get 1.0))

(event `self.ClientStartBuff`
  (params (OwningCharacter :type "ConanCharacter Object Reference") (Duration :type "Float (single-precision)"))
  (`parent.ClientStartBuff` OwningCharacter Duration)
  (bind _asis_base_bpcombat_interface (cast `/Game/Systems/Interfaces/IsBaseBPCombatInterface` (`self.OwningCharacter`)))
  (set `self.ConbatInterface` _asis_base_bpcombat_interface)
  ;[1 1 1] If we didn’t do this; then it would apply the effect twice
  (if (not (`KismetSystemLibrary.IsServer`))
    (goto _label)))

(event `self.GameplayEffectToApplyOnBuffCleared`
  (`parent.GameplayEffectToApplyOnBuffCleared`)
  (`Character.StopAnimMontage` (stale `self.GameplayEffectToApplyOnBuffStart` _asbase_player_char) "/Game/Characters/humans/animations/emotes/AM_emote_pray_sitting.AM_emote_pray_sitting" :!label _label_2)
  (`/Game/Systems/Interfaces/IsBaseBPCombatInterface.AdjustMovementSpeedMultiplier` (`self.ConbatInterface`) false (`self.SnareValue`)))

(event `self.ClientClearBuff`
  (params (OwningCharacter :type "ConanCharacter Object Reference"))
  (`parent.ClientClearBuff` OwningCharacter)
  ;[1 1 1] If we didn’t do this; then it would apply the effect twice
  (if (not (`KismetSystemLibrary.IsServer`))
    (goto _label_2)))