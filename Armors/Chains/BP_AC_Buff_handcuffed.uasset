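; Handcuffed buff that strips the player's weapons and blocks weapon changes while it is active.
; Client start unequips all weapons from the equipment inventory, while the start effect makes the buff non-expiring and sets WeaponChangeDisabled on the player character.
; Clearing the buff re-enables weapon changes.
; Client start and clear events reuse the gameplay-effect logic only when not on the server, avoiding double application.
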(event `self.InitBuff`
  (params (DamageCauser :type "Actor Object Reference") (OwningCharacter :type "ConanCharacter Object Reference") (Instigator :type "Controller Object Reference"))
  (`parent.InitBuff` null OwningCharacter Instigator)
  (bind _asis_base_bpcombat_interface (cast `/Game/Systems/Interfaces/IsBaseBPCombatInterface` (`self.OwningCharacter`)))
  (set `self.ConbatInterface` _asis_base_bpcombat_interface))

(event `EffectToApplyOnBuffTick`)

(event `self.GameplayEffectToApplyOnBuffStart`
  (`parent.GameplayEffectToApplyOnBuffStart`)
  (set `self.DoesNotExpire` true :!label _label)
  (bind _asbase_player_char (cast `/Game/Characters/BasePlayerChar` (`self.OwningCharacter`)))
  (set `ConanCharacter.WeaponChangeDisabled` true _asbase_player_char))

(event `self.ClientStartBuff`
  (params (OwningCharacter :type "ConanCharacter Object Reference") (Duration :type "Float (single-precision)"))
  (`parent.ClientStartBuff` OwningCharacter Duration)
  (bind _asbase_player_char (cast `/Game/Characters/BasePlayerChar` (`self.OwningCharacter`)))
  (`EquipmentInventory.UnequipAllWeapons` (`/Game/Characters/BaseBPChar.EquipmentInventory` _asbase_player_char))
  (bind _asis_base_bpcombat_interface (cast `/Game/Systems/Interfaces/IsBaseBPCombatInterface` (`self.OwningCharacter`)))
  (set `self.ConbatInterface` _asis_base_bpcombat_interface)
  ;[1 1 1] If we didn’t do this; then it would apply the effect twice
  (if (not (`KismetSystemLibrary.IsServer`))
    (goto _label)))

(event `self.GameplayEffectToApplyOnBuffCleared`
  (`parent.GameplayEffectToApplyOnBuffCleared`)
  (set `ConanCharacter.WeaponChangeDisabled` false (stale `self.GameplayEffectToApplyOnBuffStart` _asbase_player_char) :!label _label_2))

(event `self.ClientClearBuff`
  (params (OwningCharacter :type "ConanCharacter Object Reference"))
  (`parent.ClientClearBuff` OwningCharacter)
  ;[1 1 1] If we didn’t do this; then it would apply the effect twice
  (if (not (`KismetSystemLibrary.IsServer`))
    (goto _label_2)))